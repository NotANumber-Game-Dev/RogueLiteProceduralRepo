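; Ammo item actor that exists in the world as a dropped physics object or as a hidden equipped item, starting as Dropped on BeginPlay.
; SetAmmoState switches between the two: Dropped enables mesh physics, shadows and sphere overlap collision.
; Equipped disables physics, collision and shadows, resets the mesh's relative transform and hides it.
; SetAmmoType stores the ammo type, and the actor holds no overlap or pickup logic of its own.
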(event `self.ReceiveBeginPlay`
  (`self.setAmmoState` "NewEnumerator0"))

(fn `setAmmoState`
  (params (`New Ammo State` :type "/Game/Blueprints/Gameplay/Player/Equipment/Weapon/ENUM_WeaponState Enum" :default "NewEnumerator0"))
  (bind _skeletalmesh (`self.SkeletalMesh`))
  (bind _skeletalmesh_2 (`self.SkeletalMesh`))
  (bind _skeletalmesh_3 (`self.SkeletalMesh`))
  (bind _output_get (set `self.AmmoState` `New Ammo State`))
  (switch `/Game/Blueprints/Gameplay/Player/Equipment/Weapon/ENUM_WeaponState` _output_get
    (:`NewEnumerator0`
      (`PrimitiveComponent.SetCollisionProfileName` (`self.Sphere`) "OverlapAllDynamic" true)
      (`PrimitiveComponent.SetSimulatePhysics` _skeletalmesh_2 true)
      (`PrimitiveComponent.SetCollisionProfileName` _skeletalmesh_2 "DroppedWeapon" true)
      (`PrimitiveComponent.SetCastShadow` (`self.SkeletalMesh`) true))
    (:`NewEnumerator1`
      (`PrimitiveComponent.SetCollisionEnabled` (`self.Sphere`) "NoCollision")
      (`PrimitiveComponent.SetSimulatePhysics` _skeletalmesh_3 false)
      (`PrimitiveComponent.SetCollisionEnabled` _skeletalmesh_3 "NoCollision")
      (`SceneComponent.ResetRelativeTransform` _skeletalmesh_3)
      (`PrimitiveComponent.SetCastShadow` _skeletalmesh false)
      (`SceneComponent.SetVisibility` _skeletalmesh false true))))

(fn `setAmmoType`
  (params (`Ammo Type` :type "/Game/Blueprints/Gameplay/Player/Equipment/Weapon/ENUM_WeaponType Enum" :default "NewEnumerator0"))
  (set `self.AmmoType` `Ammo Type`))

(fn `UserConstructionScript`
  (`parent.UserConstructionScript`))