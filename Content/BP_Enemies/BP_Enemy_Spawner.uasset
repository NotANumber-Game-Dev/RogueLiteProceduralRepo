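; Enemy spawner actor that may place a single enemy at its own transform when play begins.
; A random roll against SpawnProbabilty gates spawning, then an even three-way pick chooses melee, mid-range or sniper.
; The sniper branch makes a second 0–2 integer roll against SniperSpawnProbability and falls back to mid-range on failure.
; Spawns are raised slightly above the spawner and adjust for collisions but always spawn.
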(event `self.ReceiveBeginPlay`
  (bind (_returnvalue_location _returnvalue_rotation _returnvalue_scale) (`KismetMathLibrary.BreakTransform` (`self.GetTransform`)))
  (bind (_returnvalue_location_2 _returnvalue_rotation_2 _returnvalue_scale_2) (`KismetMathLibrary.BreakTransform` (`self.GetTransform`)))
  (bind (_returnvalue_location_3 _returnvalue_rotation_3 _returnvalue_scale_3) (`KismetMathLibrary.BreakTransform` (`self.GetTransform`)))
  (if (< (`KismetMathLibrary.RandomFloatInRange` 0.0 100.0) (`self.SpawnProbabilty`))
    (switch `int` (`KismetMathLibrary.RandomIntegerInRange` 0 2)
      (:`0`
        (`|SpawnActorFromClass` (`self.Enemy_Melee`) (`KismetMathLibrary.MakeTransform` (+ _returnvalue_location (0.0 0.0 50.0)) _returnvalue_rotation _returnvalue_scale) "AdjustIfPossibleButAlwaysSpawn" "OverrideRootScale" null null))
      (:`1`
        (`|SpawnActorFromClass` (`self.Enemy_MidRange`) (`KismetMathLibrary.MakeTransform` (+ _returnvalue_location_3 (0.0 0.0 50.0)) _returnvalue_rotation_3 _returnvalue_scale_3) "AdjustIfPossibleButAlwaysSpawn" "OverrideRootScale" null null :!label _label))
      (:`2`
        (if (< (`KismetMathLibrary.RandomIntegerInRange` 0 2) (`self.SniperSpawnProbability`))
          (`|SpawnActorFromClass` (`self.Enemy_Sniper`) (`KismetMathLibrary.MakeTransform` (+ _returnvalue_location_2 (0.0 0.0 50.0)) _returnvalue_rotation_2 _returnvalue_scale_2) "AdjustIfPossibleButAlwaysSpawn" "OverrideRootScale" null null)
          (else
            (goto _label)))))))

(fn `UserConstructionScript`)