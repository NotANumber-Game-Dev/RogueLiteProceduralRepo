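; Prop actor that randomly decides at game start whether its configured static mesh appears.
; The construction script always assigns StaticMeshToSpawn to the StaticMesh component.
; On BeginPlay it rolls a percentage against Probability, reassigning the mesh on success and setting it to empty otherwise.
; A failed roll only clears the mesh; the actor itself remains.
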(event `self.ReceiveBeginPlay`
  (bind _staticmesh (`self.StaticMesh`))
  (if (< (`KismetMathLibrary.RandomFloatInRange` 0.0 100.0) (`self.Probability`))
    (`StaticMeshComponent.SetStaticMesh` _staticmesh (`self.StaticMeshToSpawn`))
    (else
      (`StaticMeshComponent.SetStaticMesh` _staticmesh null))))

(fn `UserConstructionScript`
  (`StaticMeshComponent.SetStaticMesh` (`self.StaticMesh`) (`self.StaticMeshToSpawn`)))