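; Enemy character with a configurable model that carries a weapon, shoots and takes bullet damage from the player.
; BeginPlay spawns and attaches a weapon per enemy type (sniper, melee, rifle), though all three use the same class.
; ShootPlayer limits fire rate with a Tick-accumulated timer.
; Player bullet overlaps subtract the shooter's current-slot weapon damage, turning the enemy toward the player or, at zero HP, destroying it with a chance-based weapon drop.
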(event `self.ReceiveTick`
  (params (DeltaSeconds :type "Float (single-precision)"))
  (set `self.Seconds Elapsed` (+ DeltaSeconds (`self.Seconds Elapsed`))))

(event `self.ReceiveBeginPlay`
  (bind _returnvalue_location (`KismetMathLibrary.BreakTransform` (`self.GetTransform`)))
  (bind _weapon (`self.Weapon`))
  (switch `Type` (`self.EnemyType`)
    (:`Sniper`
      (bind _returnvalue (`|SpawnActorFromClass` "/Game/Blueprints/DataBase/Weapons/BP_Iteam_Weapon_1.BP_Iteam_Weapon_1_C" (`KismetMathLibrary.MakeTransform` (0.0 0.0 0.0)) "Undefined" "OverrideRootScale" self null))
      (set `self.Weapon` _returnvalue))
    (:`Melee`
      (bind _returnvalue_2 (`|SpawnActorFromClass` "/Game/Blueprints/DataBase/Weapons/BP_Iteam_Weapon_1.BP_Iteam_Weapon_1_C" (`KismetMathLibrary.MakeTransform` (0.0 0.0 0.0)) "Undefined" "OverrideRootScale" null self))
      (set `self.Weapon` _returnvalue_2))
    (:`MidRange`
      (bind _returnvalue_3 (`|SpawnActorFromClass` "/Game/Blueprints/DataBase/Weapons/BP_Iteam_Weapon_1.BP_Iteam_Weapon_1_C" (`KismetMathLibrary.MakeTransform` (+ _returnvalue_location (0.0 0.0 50.0))) "Undefined" "OverrideRootScale" self null))
      (set `self.Weapon` _returnvalue_3)))
  (`self.K2_AttachToComponent` _weapon (`self.SkeletalMesh`) "None" "SnapToTarget" "SnapToTarget" "SnapToTarget" true)
  (`/Game/Blueprints/Gameplay/Player/Equipment/Weapon/BP_Item_Weapon.Show Mesh` _weapon)
  (`/Game/Blueprints/Gameplay/Player/Equipment/Weapon/BP_Item_Weapon.setWeaponState` _weapon "NewEnumerator1"))

(event `self.CapsuleComponent.OnComponentBeginOverlap`
  (params (OverlappedComponent :type "PrimitiveComponent Object Reference") (OtherActor :type "Actor Object Reference") (OtherComp :type "PrimitiveComponent Object Reference") (OtherBodyIndex :type Integer) (bFromSweep :type Boolean) (SweepResult :type "HitResult Structure (by ref)"))
  (bind _asbp_bullet (cast `/Game/Blueprints/Gameplay/Player/Equipment/Bullet/BP_Bullet` OtherActor))
  (bind _asbp_player (cast `/Game/Blueprints/Gameplay/Player/BP_Player` (`/Game/Blueprints/Gameplay/Player/Equipment/Bullet/BP_Bullet.WhoShoted` _asbp_bullet)))
  (bind _output_get (set `self.HP` (- (`self.HP`) (`/Game/Blueprints/Gameplay/Player/Equipment/Weapon/BP_Item_Weapon.Damage Points` (`|GetArrayItem` (`/Game/Blueprints/Gameplay/Player/BP_Player.WeaponSlot` _asbp_player) (`/Game/Blueprints/Gameplay/Player/BP_Player.CurrentWeaponSlot` _asbp_player))))))
  (`KismetSystemLibrary.PrintString` (`KismetStringLibrary.Conv_IntToString` _output_get))
  (if (<= (`self.HP`) 0)
    (`self.K2_DestroyActor`)
    (if (> (`self.Drop Probrability`) (`KismetMathLibrary.RandomFloatInRange` 0.0 100.0))
      (`/Game/Blueprints/Gameplay/Player/Equipment/Weapon/BP_Item_Weapon.setWeaponState` (`self.Weapon`) "NewEnumerator0")
      (else
        (`self.K2_DestroyActor` (`self.Weapon`))))
    (else
      (`self.K2_SetActorRotation` (`KismetMathLibrary.FindLookAtRotation` (`self.K2_GetActorLocation` self) (`self.K2_GetActorLocation` (`GameplayStatics.GetPlayerPawn` 0)))))))

(fn `Shoot Player`
  (bind _weapon (`self.Weapon`))
  (if (>= (`self.Seconds Elapsed`) (`/Game/Blueprints/Gameplay/Player/Equipment/Weapon/BP_Item_Weapon.Fire Rate` _weapon))
    (set `self.Seconds Elapsed` 0.0)
    (`/Game/Blueprints/Gameplay/Player/Equipment/Weapon/BP_Item_Weapon.Fire` _weapon (`self.ShootingCamera`) false self)
    (`/Game/Blueprints/Gameplay/Player/Equipment/Weapon/BP_Item_Weapon.Get Current Clip Ammo` _weapon)
    (`GameplayStatics.PlaySoundAtLocation` null (`self.K2_GetActorLocation`) (struct) 1.0 1.0 0.0 null null null)))

(fn `Update Walk Speed`
  (params (`Max Walk Speed` :type "Float (double-precision)"))
  (set `CharacterMovementComponent.MaxWalkSpeed` `Max Walk Speed` (`self.CharacterMovement`)))

(fn `UserConstructionScript`
  (`SkinnedMeshComponent.SetSkinnedAssetAndUpdate` (`self.Mesh`) (`self.Model`) false))