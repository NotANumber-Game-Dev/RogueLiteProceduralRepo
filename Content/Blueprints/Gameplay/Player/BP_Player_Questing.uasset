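; Player questing Blueprint that handles mission completion by taking the player out of the maze level.
; On BeginPlay it binds its completion handler to the game instance's DATABASE missions-completed event.
; The handler unloads the generated maze and its streamed level, then teleports the pawn to a hardcoded transform between loading screen show and hide calls, with no wait.
; It restores game input, unpauses and re-shows the hidden HUD after a delay.
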(event `self.ReceiveBeginPlay`
  (bind _asbp_controlled_main_game_instance (cast `/Game/Blueprints/GameModes/BP_ControlledMainGameInstance` (`GameplayStatics.GetGameInstance`)))
  (add `DATABASE.MissionsCompleted` (`/Game/Blueprints/GameModes/BP_ControlledMainGameInstance.DATABASE` _asbp_controlled_main_game_instance) (delegate `OnMissionCompleted`)))

(event `OnMissionCompleted`
  (bind _returnvalue (`GameplayStatics.GetPlayerPawn` 0))
  (bind _returnvalue_2 (`GameplayStatics.GetPlayerController` 0))
  (`KismetSystemLibrary.PrintString` "Mission completed")
  (bind _outactors (`GameplayStatics.GetAllActorsOfClass` "/Game/Blueprints/MAZE/BP_MazeGenerator.BP_MazeGenerator_C"))
  (bind _asbp_maze_generator (cast `/Game/Blueprints/MAZE/BP_MazeGenerator` (`|GetArrayItem` _outactors)))
  (`/Game/Blueprints/MAZE/BP_MazeGenerator.UnloadMap` _asbp_maze_generator)
  (bind _asbp_player (cast `/Game/Blueprints/Gameplay/Player/BP_Player` (`GameplayStatics.GetPlayerPawn` 0)))
  (`/Game/UI/WBP_HUD.Hide HUD` (`/Game/Blueprints/Gameplay/Player/BP_Player.HUD_Widget` _asbp_player))
  (bind _asbp_controlled_main_game_instance (cast `/Game/Blueprints/GameModes/BP_ControlledMainGameInstance` (`GameplayStatics.GetGameInstance`)))
  (`LevelStreaming.SetIsRequestingUnloadAndRemoval` (`/Game/Blueprints/GameModes/BP_ControlledMainGameInstance.MazeMainLevelREF` _asbp_controlled_main_game_instance) true)
  (bind _asbp_controlled_gm (cast `/Game/Blueprints/GameModes/BP_ControlledGM` (`GameplayStatics.GetGameMode`)))
  (bind _loadingscreen (`/Game/Blueprints/GameModes/BP_ControlledGM.LoadingScreen` _asbp_controlled_gm))
  (`/Game/UI/WBP_LoadingUI.Show` _loadingscreen)
  (`Actor.K2_SetActorLocation` _returnvalue (173.0 -1030.0 -6892.0) false true)
  (`Actor.K2_SetActorRotation` _returnvalue (struct :`Yaw` 90.0) false)
  (`/Game/UI/WBP_LoadingUI.Hide` _loadingscreen)
  (`WidgetBlueprintLibrary.SetInputMode_GameOnly` _returnvalue_2)
  (set `PlayerController.bShowMouseCursor` false _returnvalue_2)
  (`GameplayStatics.SetGamePaused` false)
  (`KismetSystemLibrary.Delay` 8.0)
  (bind _asbp_player_2 (cast `/Game/Blueprints/Gameplay/Player/BP_Player` (`GameplayStatics.GetPlayerPawn` 0)))
  (`/Game/UI/WBP_HUD.Show HUD` (`/Game/Blueprints/Gameplay/Player/BP_Player.HUD_Widget` _asbp_player_2)))