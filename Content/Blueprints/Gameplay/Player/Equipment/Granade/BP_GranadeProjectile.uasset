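; BP_GranadeProjectile is a grenade projectile actor that flies for a limited lifetime.
; On BeginPlay it passes its Velocity variable to the ProjectileMovement component and sizes its Sphere component to ExplosionRange.
; Tick accumulates elapsed time and destroys the actor once it exceeds LifeTime.
; The graph contains no explosion, overlap or damage logic.
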(event `self.ReceiveBeginPlay`
  (set `MovementComponent.Velocity` (`self.Velocity`) (`self.ProjectileMovement`))
  (`SphereComponent.SetSphereRadius` (`self.Sphere`) (`self.ExplosionRange`) true))

(event `self.ReceiveTick`
  (params (DeltaSeconds :type "Float (single-precision)"))
  (bind _output_get (set `self.CurrentLifeTime` (+ DeltaSeconds (`self.CurrentLifeTime`))))
  (if (> _output_get (`self.LifeTime`))
    (`self.K2_DestroyActor`)))

(fn `UserConstructionScript`)