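; Shop NPC Blueprint that opens a shop screen when interacted with.
; BeginPlay creates the WBP_Shop widget up front and stores it as BuyWidget.
; On interaction, a DoOnce adds the widget to the viewport the first time only, and every interaction calls its Show.
; Each interaction also pauses the game, switches to UI-only input and shows the mouse cursor.
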(event `self.ReceiveBeginPlay`
  (`parent.ReceiveBeginPlay`)
  (bind _returnvalue (`|CreateWidget` "/Game/UI/Components/Shop/WBP_Shop.WBP_Shop_C"))
  (set `self.BuyWidget` _returnvalue))

(event `/Game/Blueprints/Gameplay/Player/InteractionInterface/InteractionInterface.OnInteracted`
  (params (Player :type "/Game/Blueprints/Gameplay/Player/BP_Player Object Reference"))
  (bind _returnvalue (`GameplayStatics.GetPlayerController` 0))
  (bind _buywidget (`self.BuyWidget`))
  (`|ExecutionSequence`
    (:`then_0`
      (`/Engine/EditorBlueprintResources/StandardMacros.DoOnce` false
        (:`Completed`
          (`UserWidget.AddToViewport` _buywidget 0))))
    (:`then_1`
      (`/Game/UI/Components/Shop/WBP_Shop.Show` _buywidget)
      (`GameplayStatics.SetGamePaused` true)
      (`WidgetBlueprintLibrary.SetInputMode_UIOnlyEx` _returnvalue null)
      (set `PlayerController.bShowMouseCursor` true _returnvalue))))

(fn `UserConstructionScript`
  (`parent.UserConstructionScript`))