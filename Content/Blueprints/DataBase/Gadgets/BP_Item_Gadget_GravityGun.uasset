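; Gravity gun gadget item that fires a BP_GravityBullet and then goes on cooldown.
; Fire runs the parent logic, enables tick, hides the mesh, and spawns the bullet and a flash at the muzzle socket, aimed at a point along the player camera's forward vector.
; Tick advances the gadget state and times the cooldown, which UpdateHUD shows on the matching gadget slot.
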(event `self.ReceiveTick`
  (params (DeltaSeconds :type "Float (single-precision)"))
  (if (`|EnumEquality` (`self.GadgetState`) "NewEnumerator5")
    (set `self.GadgetState` "NewEnumerator4")
    (elif (`|EnumEquality` (`self.GadgetState`) "NewEnumerator4")
      (set `self.Delta Seconds` DeltaSeconds)
      (set `self.Seconds Elapsed` (+ (`self.Delta Seconds`) (`self.Seconds Elapsed`)))
      (if (> (`self.Seconds Elapsed`) (`self.Cooldown`))
        (set `self.Seconds Elapsed` 0.0)
        (`self.setGadgetState` "NewEnumerator1")))))

(fn `Fire`
  (`parent.Fire`)
  (`self.SetActorTickEnabled` true)
  (`self.hideMesh`)
  (`self.FireGravityBullet`))

(fn `FireGravityBullet`
  (bind _returnvalue (`SceneComponent.GetSocketLocation` (`self.SkeletalMesh`) "b_gun_muzzleflash"))
  (bind _asbp_player (cast `/Game/Blueprints/Gameplay/Player/BP_Player` (`GameplayStatics.GetPlayerPawn` 0)))
  (bind _camera (`/Game/Blueprints/Gameplay/Player/BP_Player.Camera` _asbp_player))
  (`|SpawnActorFromClass` "/Game/Blueprints/Gameplay/Player/Equipment/Bullet/BP_GravityBullet.BP_GravityBullet_C" (`KismetMathLibrary.MakeTransform` _returnvalue) "Undefined" "OverrideRootScale" null (* (`KismetMathLibrary.Normal` (- (+ (`SceneComponent.K2_GetComponentLocation` _camera) (* (`SceneComponent.GetForwardVector` _camera) (`self.Bullet Range`))) _returnvalue)) (* (`self.Bullet Velocity`) 1000.0)) null)
  (`|SpawnActorFromClass` "/Game/Blueprints/Gameplay/Player/Equipment/Bullet/BP_ShootFlash.BP_ShootFlash_C" (`KismetMathLibrary.MakeTransform` _returnvalue) "Undefined" "OverrideRootScale" null null))

(fn `UpdateHUD`
  (params (HUD :type "/Game/UI/WBP_HUD Object Reference") (Player :type "/Game/Blueprints/Gameplay/Player/BP_Player Object Reference"))
  (for (_array_element _array_index) (`/Game/Blueprints/Gameplay/Player/BP_Player.GadgetSlot` Player)
    (cast `/Game/Blueprints/DataBase/Gadgets/BP_Item_Gadget_GravityGun` _array_element)
    (if (`|EnumEquality` (`self.GadgetState`) "NewEnumerator4")
      (`/Game/UI/WBP_HUD.Set Cooldown Gadget` HUD _array_index (`self.Seconds Elapsed`) (`self.Cooldown`) (struct :`R` 0.756863 :`G` 0.756863 :`B` 0.756863 :`A` 0.227451))
      (break))))

(fn `UserConstructionScript`
  (`parent.UserConstructionScript`))