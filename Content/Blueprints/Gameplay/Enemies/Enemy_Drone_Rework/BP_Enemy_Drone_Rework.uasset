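; Reworked drone enemy Blueprint that overrides parent state logic for chasing and attacking the player.
; Vision alert runs toward the player, then either alerts other enemies or switches state, depending on sight.
; Attacking circles the player by rotating a radius vector over time, feeding a delayed move, then alerts allies.
; Tick prints the current state for debugging, and the attack state's sight checks do not affect its branches.
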(event `self.ReceiveTick`
  (params (DeltaSeconds :type "Float (single-precision)"))
  (`parent.ReceiveTick` DeltaSeconds)
  (`KismetSystemLibrary.PrintString` (`|GetEnumeratorNameAsString` (`self.State`))))

(fn `Rotate Around Point`
  (bind _time (`self.Time`))
  (set `self.Time` (+ (`self.Delta Seconds`) _time))
  (set `self.CurrentSpeed` (+ (* (* _time (`self.Speed`)) (select `bool` (`self.clockwise`) :`false` 1.0 :`true` -1.0 :!type "Float (single-precision)")) (`self.CurrentRotation`)))
  (`self.DELAY IN GOING POSITION` 1.0 (+ (`self.K2_GetActorLocation` (`GameplayStatics.GetPlayerPawn` 0)) (`KismetMathLibrary.RotateAngleAxis` (`KismetMathLibrary.MakeVector` (`self.radi`)) (+ (`self.Angle`) (`self.CurrentSpeed`)) (0.0 0.0 1.0)))))

(fn `StateAttacking`
  (`self.Check if Seeing Player`)
  (if true
    (set `self.CurrentSpeed` (`self.RunSpeed`))
    (`self.Rotate Around Point`)
    (`self.Delay` 0.5)
    (`self.Alert Other Enemies`)
    (set `self.State` "NewEnumerator2")
    (else
      (`self.Go to Player`)
      (`self.Check if Seeing Player`)
      (if true
        (set `self.State` "NewEnumerator2")
        (else
          (set `self.State` "NewEnumerator4"))))))

(fn `StateVisionAlert`
  (set `self.CurrentSpeed` (`self.RunSpeed`))
  (`self.Go to Player`)
  (bind _seeplayer (`self.Check if Seeing Player`))
  (if _seeplayer
    (`self.Alert Other Enemies`)
    (set `self.State` "NewEnumerator2")
    (else
      (set `self.State` "NewEnumerator4"))))

(fn `UserConstructionScript`
  (`parent.UserConstructionScript`))