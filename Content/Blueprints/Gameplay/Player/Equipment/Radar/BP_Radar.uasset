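; BP_Radar is a player equipment actor that periodically detects nearby enemies for a radar.
; Tick accumulates time and, at each refresh interval, gathers every BP_Enemy_REWORK within the radar radius of the player pawn.
; It rebuilds the enemy and cosine arrays and prints debug values, while the sine array only grows with zeros.
; The angle function is a stub returning zero, so no real bearing is computed.
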(event `self.ReceiveTick`
  (params (DeltaSeconds :type "Float (single-precision)"))
  (bind _output_get (set `self.temps acumulat` (+ (`self.temps acumulat`) DeltaSeconds)))
  (if (>= _output_get (`self.temps refresh`))
    (set `self.temps acumulat` 0.0)
    (bind _output_get_2 (set `self.enemy in range` (`self.enemy in range`)))
    (`KismetArrayLibrary.Array_Clear` _output_get_2)
    (bind _output_get_3 (set `self.ArrayEnemyCos` (`self.ArrayEnemyCos`)))
    (`KismetArrayLibrary.Array_Clear` _output_get_3)
    (bind _outactors (`GameplayStatics.GetAllActorsOfClass` "/Game/Blueprints/Gameplay/Enemies/REWORK/BP_Enemy_REWORK.BP_Enemy_REWORK_C"))
    (for _array_element _outactors
      (if (<= (`KismetMathLibrary.Vector_Distance` (`self.K2_GetActorLocation` _array_element) (`self.K2_GetActorLocation` (`GameplayStatics.GetPlayerPawn` 0))) (`self.Radi Radar`))
        (bind _output_get_4 (set `self.enemy in range` (`self.enemy in range`)))
        (`KismetArrayLibrary.Array_Add` _output_get_4 _array_element)
        (bind _angle (`self.Angle Between 2 Vectors` (`self.K2_GetActorLocation` (`GameplayStatics.GetPlayerPawn` 0)) (`self.K2_GetActorLocation` _array_element)))
        (bind _output_get_5 (set `self.ArrayEnemyCos` (`self.ArrayEnemyCos`)))
        (`KismetArrayLibrary.Array_Add` _output_get_5 _angle)
        (bind _output_get_6 (set `self.ArrayEnemySin` (`self.ArrayEnemySin`)))
        (`KismetArrayLibrary.Array_Add` _output_get_6)
        (`KismetSystemLibrary.PrintString` (`KismetStringLibrary.Concat_StrStr` (`KismetStringLibrary.Concat_StrStr` (`KismetStringLibrary.Conv_DoubleToString` _angle) " / ") (`KismetStringLibrary.Conv_DoubleToString` 0.0)))))))

(fn `Angle Between 2 Vectors`
  (params (`Position Player` :type "Vector Structure (by ref)") (`Position Enemy` :type "Vector Structure (by ref)"))
  (returns (Angle :type "Float (double-precision)"))
  (locals (R :type "Float (double-precision)" :default 0.0) (X :type "Float (double-precision)") (Y :type "Float (double-precision)"))
  (return 0.0))

(fn `UserConstructionScript`)