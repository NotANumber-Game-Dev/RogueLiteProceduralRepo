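; BP_PopUp is a placed actor that shows a one-time pop-up of text and images to the player.
; WaitForLevelLoad selects the trigger: the BP_ControlledGM finished-loading event, or BP_Player overlapping the actor.
; After a configurable delay, it creates WBP_PopUp, passes itself and the content array, then pauses the game with UI-only input focused on the widget.
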(event `self.ReceiveBeginPlay`
  (if (`self.Wait for Level Load?`)
    (bind _asbp_controlled_gm (cast `/Game/Blueprints/GameModes/BP_ControlledGM` (`GameplayStatics.GetGameMode`)))
    (add `/Game/Blueprints/GameModes/BP_ControlledGM.Finished Loading Event` _asbp_controlled_gm (delegate `Finished Loading Event_Event_0`))))

(event `Finished Loading Event_Event_0`
  (`/Engine/EditorBlueprintResources/StandardMacros.DoOnce` false :!label _label
    (:`Completed`
      (`KismetSystemLibrary.Delay` (`self.Delayed Aperiance`))
      (bind _returnvalue (`|CreateWidget` "/Game/UI/Components/PopUps/WBP_PopUp.WBP_PopUp_C" (`GameplayStatics.GetPlayerController` 0)))
      (bind _output_get (set `self.PopUp` _returnvalue))
      (`UserWidget.AddToViewport` _output_get 200)
      (`/Game/UI/Components/PopUps/WBP_PopUp.SetInstigator` _output_get self)
      (`/Game/UI/Components/PopUps/WBP_PopUp.SetArrayPopUps` _output_get (`self.TextAndImgToDisplay`))
      (`/Game/UI/Components/PopUps/WBP_PopUp.Show` _output_get)
      (`GameplayStatics.SetGamePaused` true)
      (`WidgetBlueprintLibrary.SetInputMode_UIOnlyEx` (`GameplayStatics.GetPlayerController` 0) (`self.PopUp`)))))

(event `self.ReceiveActorBeginOverlap`
  (params (OtherActor :type "Actor Object Reference"))
  (if (not (`self.Wait for Level Load?`))
    (cast `/Game/Blueprints/Gameplay/Player/BP_Player` OtherActor)
    (goto _label)))

(fn `UserConstructionScript`)