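; BP_Luz_ToFollow is a maze light prop Blueprint with a point light that can be switched on and off.
; The construction script caches the light's configured intensity.
; ToggleLights flips an active flag and sets the intensity to the cached value or zero, so the component itself is never hidden.
; Nothing in this Blueprint calls the toggle, and its Tick event is empty.
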(event `self.ReceiveTick`
  (params (DeltaSeconds :type "Float (single-precision)")))

(fn `Toggle Lights`
  (bind _is_active (`self.Is Active`))
  (set `self.Is Active` (not _is_active))
  (if _is_active
    (`LightComponent.SetIntensity` (`self.PointLight`) (`self.Intensity`))
    (else
      (`LightComponent.SetIntensity` (`self.PointLight`) 0.0))))

(fn `UserConstructionScript`
  (set `self.Intensity` (`LightComponentBase.Intensity` (`self.PointLight`))))