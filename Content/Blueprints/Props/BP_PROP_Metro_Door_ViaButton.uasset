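; Metro door prop that slides open once its linked button, WhatButton, has been activated.
; Tick polls the button every frame and plays the SlidingDoor timeline, which moves the Door's relative location.
; A DoOnce on the timeline update plays an attenuated opening sound only the first time.
; When the player leaves the Box, the timeline reverses unless KeepOpen is set, though Tick keeps calling Play while the button remains activated.
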(event `self.ReceiveTick`
  (params (DeltaSeconds :type "Float (single-precision)"))
  (`self.OpenDoor`))

(event `OpenDoor`
  (bind _whatbutton_ (`self.WhatButton?`))
  (`/Engine/EditorBlueprintResources/StandardMacros.IsValid` _whatbutton_
    (:`Is Valid`
      (if (`/Game/Blueprints/Props/BP_Button.Has Been Activated` _whatbutton_)
        (bind (_direction _sliding_door) (`Timeline|SlidingDoor` :`NewTime` 1.0 :!label _label)
          (:`Update`
            (`SceneComponent.K2_SetRelativeLocation` (`self.Door`) (+ _sliding_door (0.0 0.0 109.0)) false false)
            (`/Engine/EditorBlueprintResources/StandardMacros.DoOnce` false
              (:`Completed`
                (`GameplayStatics.SpawnSoundAtLocation` "/Game/Sounds/Effects/OpeningDoorEffect.OpeningDoorEffect" (`self.K2_GetActorLocation`) (struct) 1.0 1.0 0.0 "/Game/Sounds/Effects/SA_Attenuation.SA_Attenuation" null)))))))))

(event `self.Box.OnComponentEndOverlap`
  (params (OverlappedComponent :type "PrimitiveComponent Object Reference") (OtherActor :type "Actor Object Reference") (OtherComp :type "PrimitiveComponent Object Reference") (OtherBodyIndex :type Integer))
  (if (not (`self.Keep Open?`))
    (cast `/Game/Blueprints/Gameplay/Player/BP_Player` OtherActor)
    (goto _label :!via `Reverse`)))

(fn `UserConstructionScript`)