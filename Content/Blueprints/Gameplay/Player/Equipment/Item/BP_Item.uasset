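; BP_Item is an interactable equipment item actor with a generic "Interact" prompt and an inventory representation.
; Interaction range events set and show that prompt as a tooltip on the player's HUD widget, then hide it on exit.
; It exposes its scene root as the prompt's attach component.
; ReturnUIWidget builds an inventory item widget showing the item's UI texture.
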(event `/Game/Blueprints/Gameplay/Player/InteractionInterface/InteractionInterface.OnIteractionRangeEntered`
  (params (Player :type "/Game/Blueprints/Gameplay/Player/BP_Player Object Reference"))
  (bind _hud_widget (`/Game/Blueprints/Gameplay/Player/BP_Player.HUD_Widget` Player))
  (`/Game/UI/WBP_HUD.Set Tooltip` _hud_widget (`self.getInteractionText`))
  (`/Game/UI/WBP_HUD.Show Tooltip` _hud_widget))

(event `/Game/Blueprints/Gameplay/Player/InteractionInterface/InteractionInterface.OnInteractionRangeExited`
  (`/Game/UI/WBP_HUD.Hide Tooltip` (`/Game/Blueprints/Gameplay/Player/BP_Player.HUD_Widget` (stale `/Game/Blueprints/Gameplay/Player/InteractionInterface/InteractionInterface.OnIteractionRangeEntered` Player))))

(fn `getInteractionText`
  (returns (Text :type Text))
  (return "Interact"))

(fn `getInteractionTextAttached`
  (returns (AttachedComponent :type "SceneComponent Object Reference"))
  (return (`self.DefaultSceneRoot`)))

(fn `Return UI Widget`
  (returns (`Item Widget` :type "/Game/UI/Components/Game/Inventory/WBP_Inventory_Item Object Reference"))
  (bind _returnvalue (`|CreateWidget` "/Game/UI/Components/Game/Inventory/WBP_Inventory_Item.WBP_Inventory_Item_C"))
  (`/Game/UI/Components/Game/Inventory/WBP_Inventory_Item.Set Image` _returnvalue (`self.UI_ShowTexture`))
  (return _returnvalue))

(fn `UserConstructionScript`)