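; Gadget item that temporarily gives the player's current weapon explosive bullets, then goes on cooldown.
; Fire enables Tick, hides the mesh, remembers the current weapon slot and sets its ExplosiveBullets flag.
; Tick times the active state, clears the flag on that remembered slot when Duration expires, then times Cooldown before switching state again.
; UpdateHUD finds the gadget's slot by class, showing remaining duration or elapsed cooldown.
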(event `self.ReceiveBeginPlay`
  (set `self.Duration` 10.0))

(event `self.ReceiveTick`
  (params (DeltaSeconds :type "Float (single-precision)"))
  (set `self.Delta Seconds` DeltaSeconds)
  (if (`|EnumEquality` (`self.GadgetState`) "NewEnumerator5")
    (set `self.Seconds Elapsed` (+ (`self.Delta Seconds`) (`self.Seconds Elapsed`)))
    (if (> (`self.Seconds Elapsed`) (`self.Duration`))
      (bind _asbp_player (cast `/Game/Blueprints/Gameplay/Player/BP_Player` (`GameplayStatics.GetPlayerPawn` 0)))
      (set `/Game/Blueprints/Gameplay/Player/Equipment/Weapon/BP_Item_Weapon.ExplosiveBullets` false (`|GetArrayItem` (`/Game/Blueprints/Gameplay/Player/BP_Player.WeaponSlot` _asbp_player) (`self.WeaponCheatedIndex`)))
      (`self.setGadgetState` "NewEnumerator4")
      (set `self.Seconds Elapsed` 0.0))
    (elif (`|EnumEquality` (`self.GadgetState`) "NewEnumerator4")
      (set `self.Seconds Elapsed` (+ (`self.Delta Seconds`) (`self.Seconds Elapsed`)))
      (if (> (`self.Seconds Elapsed`) (`self.Cooldown`))
        (set `self.Seconds Elapsed` 0.0)
        (`self.setGadgetState` "NewEnumerator1")))))

(fn `Fire`
  (`parent.Fire`)
  (`self.SetActorTickEnabled` true)
  (bind _asbp_player (cast `/Game/Blueprints/Gameplay/Player/BP_Player` (`GameplayStatics.GetPlayerPawn` 0)))
  (bind _currentweaponslot (`/Game/Blueprints/Gameplay/Player/BP_Player.CurrentWeaponSlot` _asbp_player))
  (set `self.WeaponCheatedIndex` _currentweaponslot)
  (set `/Game/Blueprints/Gameplay/Player/Equipment/Weapon/BP_Item_Weapon.ExplosiveBullets` true (`|GetArrayItem` (`/Game/Blueprints/Gameplay/Player/BP_Player.WeaponSlot` _asbp_player) _currentweaponslot))
  (`self.hideMesh`))

(fn `UpdateHUD`
  (params (HUD :type "/Game/UI/WBP_HUD Object Reference") (Player :type "/Game/Blueprints/Gameplay/Player/BP_Player Object Reference"))
  (bind _gadgetstate (`self.GadgetState`))
  (bind _duration (`self.Duration`))
  (for (_array_element _array_index) (`/Game/Blueprints/Gameplay/Player/BP_Player.GadgetSlot` Player)
    (cast `/Game/Blueprints/DataBase/Gadgets/BP_Item_Gadget_ExplosiveAmmo` _array_element)
    (if (`|EnumEquality` _gadgetstate "NewEnumerator5")
      (`/Game/UI/WBP_HUD.Set Cooldown Gadget` HUD _array_index (- _duration (`self.Seconds Elapsed`)) _duration (struct :`R` 0.756863 :`G` 0.756863 :`B` 0.756863 :`A` 0.227451))
      (break)
      (elif (`|EnumEquality` _gadgetstate "NewEnumerator4")
        (`/Game/UI/WBP_HUD.Set Cooldown Gadget` HUD _array_index (`self.Seconds Elapsed`) (`self.Cooldown`) (struct :`R` 0.756863 :`G` 0.756863 :`B` 0.756863 :`A` 0.227451))
        (break)))))

(fn `UserConstructionScript`
  (`parent.UserConstructionScript`))