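; Melee enemy that overrides parent state functions to react on sighting the player, chase at run speed and attack at close range.
; BeginPlay caches the hidden HP bar widget and melee animation instance, picking a random attack animation.
; The chase state switches state by 2D distance to the player.
; Attacking flags the animation, waits the attack delay, fires the Weapon as a non-player, then rerolls the animation and changes state.
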(event `self.ReceiveBeginPlay`
  (`parent.ReceiveBeginPlay`)
  (bind _aswbp_hpbar_enemies (cast `/Game/UI/WBP_HPBarEnemies` (`WidgetComponent.GetWidget` (`self.Widget`))))
  (bind _output_get (set `self.HPBarWidget` _aswbp_hpbar_enemies))
  (`Widget.SetVisibility` _output_get "Hidden")
  (bind _asbp_anim_enemy_cac (cast `/Game/Models/SkeletalMeshes/Enemies/CaC/Animation/BP_Anim_Enemy_CAC` (`SkeletalMeshComponent.GetAnimInstance` (`self.Mesh`))))
  (set `/Game/Models/SkeletalMeshes/Enemies/CaC/Animation/BP_Anim_Enemy_CAC.AnimationAttackIndex` (`KismetMathLibrary.RandomIntegerInRange` 0 4) _asbp_anim_enemy_cac)
  (set `self.BP Anim CAC` _asbp_anim_enemy_cac))

(event `MeleeFire`
  (set `/Game/Models/SkeletalMeshes/Enemies/CaC/Animation/BP_Anim_Enemy_CAC.IsAttacking` true (`self.BP Anim CAC`))
  (`KismetSystemLibrary.Delay` (`self.Attack Time Rate`))
  (`/Game/Blueprints/Gameplay/Player/Equipment/Weapon/BP_Item_Weapon.Fire` (`self.Weapon`) (`self.Shooting Camera`) false self)
  (set `/Game/Models/SkeletalMeshes/Enemies/CaC/Animation/BP_Anim_Enemy_CAC.AnimationAttackIndex` (`KismetMathLibrary.RandomIntegerInRange` 0 4) (`self.BP Anim CAC`))
  (set `self.State` "NewEnumerator1"))

(fn `StateAttacking`
  (`self.MeleeFire`))

(fn `StateChasePlayer`
  (set `/Game/Models/SkeletalMeshes/Enemies/CaC/Animation/BP_Anim_Enemy_CAC.IsAttacking` false (`self.BP Anim CAC`))
  (`self.UpdateWalkSpeed` (`self.RunSpeed`))
  (`self.Go to Player`)
  (if (<= (`KismetMathLibrary.Vector_Distance2D` (`self.K2_GetActorLocation` (`GameplayStatics.GetPlayerPawn` 0)) (`self.K2_GetActorLocation`)) 150.0)
    (set `self.State` "NewEnumerator2")
    (else
      (set `self.State` "NewEnumerator1"))))

(fn `StateVisionAlert`
  (set `/Game/Models/SkeletalMeshes/Enemies/CaC/Animation/BP_Anim_Enemy_CAC.IsAttacking` false (`self.BP Anim CAC`))
  (`self.UpdateWalkSpeed` (`self.RunSpeed`))
  (`self.RotateToPlayer` true)
  (bind _seeplayer (`self.Check if Seeing Player`))
  (if _seeplayer
    (`self.Go to Player`)
    (`self.RotateToPlayer` true)
    (set `self.State` "NewEnumerator15")
    (else
      (set `self.LastSeenPlayerPosition` (`self.K2_GetActorLocation` (`GameplayStatics.GetPlayerPawn` 0)))
      (set `self.State` "NewEnumerator10"))))

(fn `UserConstructionScript`
  (`parent.UserConstructionScript`))