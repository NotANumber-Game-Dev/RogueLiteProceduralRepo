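; BP_SpawnLevelDetail reads an XML file on BeginPlay and prints its content to screen; despite its name, it spawns nothing.
; The file path combines the project content directory with the XmlPath variable.
; It stores the parsed tags, child tags, content and child content in variables, but only loops over the top-level content for printing.
; The construction script is empty.
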(event `self.ReceiveBeginPlay`
  (`self.ReadXmlFile` (`KismetStringLibrary.Concat_StrStr` (`KismetSystemLibrary.GetProjectContentDirectory`) (`self.Xml Path`)))
  (bind _var (`self.getTag`))
  (set `self.XMLTags` _var)
  (bind _var_2 (`self.getChildTag`))
  (set `self.XMLChildrenTags` _var_2)
  (bind _var_3 (`self.getContent`))
  (set `self.XMLContent` _var_3)
  (bind _var_4 (`self.getChildContent`))
  (set `self.XMLChildContent` _var_4)
  (for _array_element (`self.XMLContent`)
    (`KismetSystemLibrary.PrintString` _array_element true true (struct :`G` 0.66 :`B` 1.0 :`A` 1.0) 5.0)))

(fn `UserConstructionScript`)