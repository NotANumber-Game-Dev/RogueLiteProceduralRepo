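; BP_Item_Stackable is an item Blueprint for stackable player equipment that supplies its own inventory UI entry.
; On BeginPlay it creates a WBP_Inventory_Item widget, caches it as InventoryUI and sets its image from UIShowTexture.
; ReturnUIWidget copies the Ammo count into the widget's Amount, refreshes the display and returns that cached widget.
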(event `self.ReceiveBeginPlay`
  (bind _returnvalue (`|CreateWidget` "/Game/UI/Components/Game/Inventory/WBP_Inventory_Item.WBP_Inventory_Item_C"))
  (bind _output_get (set `self.Inventory UI` _returnvalue))
  (`/Game/UI/Components/Game/Inventory/WBP_Inventory_Item.Set Image` _output_get (`self.UI_ShowTexture`)))

(fn `Return UI Widget`
  (returns (`Item Widget` :type "/Game/UI/Components/Game/Inventory/WBP_Inventory_Item Object Reference"))
  (bind _inventory_ui (`self.Inventory UI`))
  (set `/Game/UI/Components/Game/Inventory/WBP_Inventory_Item.Amount` (`self.Ammo`) _inventory_ui)
  (`/Game/UI/Components/Game/Inventory/WBP_Inventory_Item.Update Amount` _inventory_ui)
  (return _inventory_ui))

(fn `UserConstructionScript`
  (`parent.UserConstructionScript`))