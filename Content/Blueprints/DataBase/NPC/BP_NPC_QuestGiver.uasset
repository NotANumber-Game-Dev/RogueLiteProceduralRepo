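; Quest giver NPC Blueprint that shows a quest UI and can send the player into a game level.
; ExecUIRelated extends the parent and, behind a DoOnce, creates the quest giver widget, binds its button, pauses the game and switches to UI-only input.
; EnterLevelWithSetings removes the widget and player HUD, re-enables camera rotation, smooth-loads GameLevel through the game instance and restores game-only input.
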(fn `Enter Level With Setings`
  (bind _returnvalue (`GameplayStatics.GetPlayerController` 0))
  (`Widget.RemoveFromParent` (`self.UI Related`))
  (bind _asbp_player (cast `/Game/Blueprints/Gameplay/Player/BP_Player` (`GameplayStatics.GetPlayerPawn` 0)))
  (set `/Game/Blueprints/Gameplay/Player/BP_Player.canRotateCamara` true _asbp_player)
  (`Widget.RemoveFromParent` (`/Game/Blueprints/Gameplay/Player/BP_Player.HUD_Widget` _asbp_player))
  (bind _asbp_controlled_main_game_instance (cast `/Game/Blueprints/GameModes/BP_ControlledMainGameInstance` (`GameplayStatics.GetGameInstance`)))
  (`/Game/Blueprints/GameModes/BP_ControlledMainGameInstance.Call Smooth Load Level` _asbp_controlled_main_game_instance (`self.GameLevel`) false false)
  (`WidgetBlueprintLibrary.SetInputMode_GameOnly` _returnvalue)
  (set `PlayerController.bShowMouseCursor` false _returnvalue))

(fn `ExecUIRelated`
  (bind _returnvalue (`GameplayStatics.GetPlayerController` 0))
  (`parent.ExecUIRelated`)
  (`|ExecutionSequence`
    (:`then_0`
      (`/Engine/EditorBlueprintResources/StandardMacros.DoOnce` false
        (:`Completed`
          (bind _returnvalue_2 (`|CreateWidget` "/Game/UI/WBP_NPC_QuestGiver.WBP_NPC_QuestGiver_C"))
          (bind _output_get (set `self.UI Related` _returnvalue_2))
          (add `Button.OnClicked` (`/Game/UI/Components/Button/WBP_Button.ButtonElement` (`/Game/UI/WBP_NPC_QuestGiver.WBP_Button` _output_get)) (`|CreateDelegate` :!event `Enter Level With Setings`))
          (`UserWidget.AddToViewport` _returnvalue_2 0)
          (`GameplayStatics.SetGamePaused` true)
          (`WidgetBlueprintLibrary.SetInputMode_UIOnlyEx` _returnvalue _returnvalue_2)
          (set `PlayerController.bShowMouseCursor` true _returnvalue))))))

(fn `UserConstructionScript`
  (`parent.UserConstructionScript`))