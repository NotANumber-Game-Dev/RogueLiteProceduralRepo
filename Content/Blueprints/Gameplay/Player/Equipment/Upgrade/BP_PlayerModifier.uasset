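; BP_PlayerModifier is a player equipment upgrade modifier holding stat values for health, shield, velocity, damage, knockback and recoil.
; Its SetRandomValues function rolls each stat independently within one shared range, using integers for most and floats for velocity and recoil.
; The graph only assigns these values and does not apply them to the player.
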(fn `setRandomValues`
  (set `self.HP` (`KismetMathLibrary.RandomIntegerInRange` 0 100))
  (set `self.Shield` (`KismetMathLibrary.RandomIntegerInRange` 0 100))
  (set `self.Vel` (`KismetMathLibrary.RandomFloatInRange` 0.0 100.0))
  (set `self.Dmg` (`KismetMathLibrary.RandomIntegerInRange` 0 100))
  (set `self.Knokback` (`KismetMathLibrary.RandomIntegerInRange` 0 100))
  (set `self.Recoil` (`KismetMathLibrary.RandomFloatInRange` 0.0 100.0)))