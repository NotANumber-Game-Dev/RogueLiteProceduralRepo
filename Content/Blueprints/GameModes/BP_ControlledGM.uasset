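; Game mode that runs level streaming behind a fading loading screen.
; On BeginPlay it creates the loading widget and registers its loading system with the main game instance.
; SmoothLoadLevel fades in, optionally unloads the current level, loads a streamed level or level instance, then fades out and signals completion.
; A LevelGeneration instance loaded without unloading is also stored on the game instance as the maze main level.
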(event `self.ReceiveBeginPlay`
  (bind _returnvalue (`GameplayStatics.GetGameInstance`))
  (`KismetSystemLibrary.PrintString` "Acces GM" false)
  (`/Engine/EditorBlueprintResources/StandardMacros.IsValid` _returnvalue
    (:`Is Valid`
      (bind _asbp_controlled_main_game_instance (cast `/Game/Blueprints/GameModes/BP_ControlledMainGameInstance` _returnvalue))
      (add `/Game/Blueprints/GameModes/BP_ControlledMainGameInstance.SmoothLoadLevel` _asbp_controlled_main_game_instance (delegate `SmoothLoadLevel`))
      (bind _returnvalue_2 (`|CreateWidget` "/Game/UI/WBP_LoadingUI.WBP_LoadingUI_C" (`GameplayStatics.GetPlayerController` 0)))
      (`/Engine/EditorBlueprintResources/StandardMacros.DoOnce` false
        (:`Completed`
          (set `self.LoadingScreen` _returnvalue_2))))))

(event `SmoothLoadLevel`
  (params (LevelName :type Name) (UsePersistentLevels :type Boolean) (`Unload current` :type Boolean))
  (`/Game/UI/WBP_LoadingUI.Fade In` (`self.LoadingScreen`) (delegate `StartLoading`)))

(event `StartLoading`
  (if (stale `SmoothLoadLevel` `Unload current`)
    (`GameplayStatics.UnloadStreamLevel` (`self.Current Level`))
    (bind _output_get (set `self.Current Level` (stale `SmoothLoadLevel` LevelName)))
    (if (stale `SmoothLoadLevel` UsePersistentLevels)
      (`GameplayStatics.LoadStreamLevel` _output_get true true)
      (else
        (`LevelStreamingDynamic.LoadLevelInstance` (`KismetStringLibrary.Conv_NameToString` _output_get))))
    (elif (stale `SmoothLoadLevel` UsePersistentLevels)
      (`GameplayStatics.LoadStreamLevel` (stale `SmoothLoadLevel` LevelName) true true)
      (else
        (bind (_boutsuccess _returnvalue) (`LevelStreamingDynamic.LoadLevelInstance` (`KismetStringLibrary.Conv_NameToString` (stale `SmoothLoadLevel` LevelName))))
        (if (== (stale `SmoothLoadLevel` LevelName) "LevelGeneration")
          (bind _asbp_controlled_main_game_instance (cast `/Game/Blueprints/GameModes/BP_ControlledMainGameInstance` (`GameplayStatics.GetGameInstance`)))
          (set `/Game/Blueprints/GameModes/BP_ControlledMainGameInstance.MazeMainLevelREF` _returnvalue _asbp_controlled_main_game_instance)))))
  (`/Game/UI/WBP_LoadingUI.Fade Out` (`self.LoadingScreen`) (delegate `Finished Loading`)))

(event `Finished Loading`
  (`self.Finished Loading Event`))

(fn `UserConstructionScript`)