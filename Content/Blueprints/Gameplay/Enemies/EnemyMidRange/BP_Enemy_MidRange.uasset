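; Mid-range enemy character that gets randomized combat traits for each instance.
; The construction script sets the mannequin mesh, rolls weapon, HP, accuracy, vision range and sound range within set bounds, and grants a grenade by probability.
; BeginPlay copies HP into the current-health float, and a helper function changes max walk speed.
; The Hit event is empty, and leftover nodes for zeroing health and facing the player are unconnected.
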(event `self.ReceiveBeginPlay`
  (set `self.HP_Actual` (`KismetMathLibrary.Conv_IntToDouble` (`self.HP`))))

(event `self.ReceiveHit`
  (params (MyComp :type "PrimitiveComponent Object Reference") (Other :type "Actor Object Reference") (OtherComp :type "PrimitiveComponent Object Reference") (bSelfMoved :type Boolean) (HitLocation :type "Vector Structure") (HitNormal :type "Vector Structure") (NormalImpulse :type "Vector Structure") (Hit :type "HitResult Structure (by ref)")))

(fn `UpdateWalkSpeed`
  (params (NewWalkSpeed :type "Float (double-precision)"))
  (set `CharacterMovementComponent.MaxWalkSpeed` NewWalkSpeed (`self.CharacterMovement`)))

(fn `UserConstructionScript`
  (`SkinnedMeshComponent.SetSkinnedAssetAndUpdate` (`self.Mesh`) "/Game/Mannequin/Character/Mesh/SK_Mannequin.SK_Mannequin" false)
  (set `self.EnemyWeapon` (cast `Weapon` (`KismetMathLibrary.Conv_IntToByte` (`KismetMathLibrary.RandomIntegerInRange` 0 2))))
  (set `self.HP` (`KismetMathLibrary.RandomIntegerInRange` (`self.HP_Min`) (`self.HP_Max`)))
  (set `self.Accuracy` (`KismetMathLibrary.RandomIntegerInRange` (`self.Accuracy_Min`) (`self.Accuracy_Max`)))
  (set `self.VisionRange` (`KismetMathLibrary.RandomIntegerInRange` (`self.VisionRange_Min`) (`self.VisionRange_Max`)))
  (set `self.SoundRange` (`KismetMathLibrary.RandomIntegerInRange` (`self.SoundRange_Min`) (`self.SoundRange_Max`)))
  (if (< (`KismetMathLibrary.RandomIntegerInRange` 0 100) (`self.ProbGranade`))
    (set `self.Granade` true)))