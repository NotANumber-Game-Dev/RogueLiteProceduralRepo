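; Location_BP is a quest objective actor that completes a quest when the player walks into its box trigger.
; On overlap, it checks the player's active quests for one whose ActorReference points to this actor and calls QuestComplete on the player.
; It then searches all BP_NPC_QuestGiver actors and fires EventQuestComplete on those whose quest name matches.
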(event `self.Box.OnComponentBeginOverlap`
  (params (OverlappedComponent :type "PrimitiveComponent Object Reference") (OtherActor :type "Actor Object Reference") (OtherComp :type "PrimitiveComponent Object Reference") (OtherBodyIndex :type Integer) (bFromSweep :type Boolean) (SweepResult :type "HitResult Structure (by ref)"))
  (bind _asbp_player (cast `/Game/Blueprints/Gameplay/Player/BP_Player` OtherActor))
  (for _array_element (`/Game/Blueprints/Gameplay/Player/BP_Player.ActiveQuests` _asbp_player)
    (bind (_questinfo_questname _questinfo_questdescription _questinfo_actorreference) (break `/Game/Blueprints/DataBase/Quest/QuestInfo` (`/Game/Blueprints/DataBase/Quest/BP_Quest.QuestInfo` _array_element)))
    (if (== self _questinfo_actorreference)
      (`/Game/Blueprints/Gameplay/Player/BP_Player.QuestComplete` _asbp_player _array_element)
      (bind _outactors (`GameplayStatics.GetAllActorsOfClass` "/Game/Blueprints/DataBase/NPC/BP_NPC_QuestGiver.BP_NPC_QuestGiver_C"))
      (for _array_element_2 _outactors
        (bind _questinforef_questname (break `/Game/Blueprints/DataBase/Quest/QuestInfo` (`/Game/Blueprints/DataBase/NPC/BP_NPC_QuestGiver.QuestInfoRef` _array_element_2)))
        (if (`KismetTextLibrary.EqualEqual_TextText` _questinfo_questname _questinforef_questname)
          (`/Game/Blueprints/DataBase/NPC/BP_NPC_QuestGiver.EventQuestComplete` _array_element_2))))))

(fn `UserConstructionScript`)