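; Deployable turret gadget that detaches with physics on use and auto-fires at nearby enemies for a limited time, then cools down.
; BeginPlay spawns a turret pawn as bullet instigator and a turret weapon attached to the rotating cannon.
; While active, Tick scans the detection sphere, line-traces for clear sight, aims at a retained target and fires at the weapon's rate.
; The target resets when it leaves overlap or the active time ends.
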(event `self.ReceiveActorEndOverlap`
  (params (OtherActor :type "Actor Object Reference"))
  (if (== OtherActor (`self.Objective`))
    (set `self.Objective` (`self.NewObjective`))))

(event `self.ReceiveBeginPlay`
  (`parent.ReceiveBeginPlay`)
  (bind _returnvalue (`|SpawnActorFromClass` "/Game/Blueprints/Gameplay/Player/Equipment/Gadget/Turrent/BP_Pawn_Turret.BP_Pawn_Turret_C" (`SceneComponent.K2_GetComponentToWorld` (`self.CanyoGiretori`)) "AlwaysSpawn" "OverrideRootScale" self null))
  (bind _output_get (set `self.Bullet Instigator` _returnvalue))
  (bind _returnvalue_2 (`|SpawnActorFromClass` "/Game/Blueprints/DataBase/Gadgets/BP_Item_Weapon_TurreT.BP_Item_Weapon_Turret_C" (`SceneComponent.K2_GetComponentToWorld` (`self.CanyoGiretori`)) "AlwaysSpawn" "OverrideRootScale" _output_get null))
  (bind _output_get_2 (set `/Game/Blueprints/Gameplay/Player/Equipment/Gadget/Turrent/BP_Pawn_Turret.Weapon Asigned` _returnvalue_2 _returnvalue))
  (set `self.Turret Weapon` _output_get_2)
  (`/Game/Blueprints/Gameplay/Player/Equipment/Weapon/BP_Item_Weapon.setWeaponState` _returnvalue_2 "NewEnumerator1")
  (`self.K2_AttachToComponent` _returnvalue_2 (`self.CanyoGiretori`) "None" "SnapToTarget" "SnapToTarget" "SnapToTarget" true)
  (set `PrimitiveComponent.bGenerateOverlapEvents` false (`self.RadiDeVigilancia`))
  (set `self.Cooldown` 3.0))

(event `self.ReceiveTick`
  (params (DeltaSeconds :type "Float (single-precision)"))
  (bind _gadgetstate (`self.GadgetState`))
  (set `self.Delta Seconds` DeltaSeconds)
  (if (`|EnumEquality` _gadgetstate "NewEnumerator5")
    (if (>= (`self.Duration`) (`self.TimeActive`))
      (set `self.Seconds Elapsed` (+ (`self.Delta Seconds`) (`self.Seconds Elapsed`)))
      (set `self.TimeActive` (+ (`self.TimeActive`) (`self.Delta Seconds`)))
      (set `PrimitiveComponent.bGenerateOverlapEvents` true (`self.RadiDeVigilancia`))
      (for _array_element (`PrimitiveComponent.GetOverlappingActors` (`self.RadiDeVigilancia`) "/Game/Blueprints/Gameplay/Enemies/REWORK/BP_Enemy_REWORK.BP_Enemy_REWORK_C")
        (bind _asbp_enemy_rework (cast `/Game/Blueprints/Gameplay/Enemies/REWORK/BP_Enemy_REWORK` _array_element))
        (bind (_outhit _returnvalue) (`KismetSystemLibrary.LineTraceSingle` (`self.K2_GetActorLocation` (`self.Turret Weapon`)) (`self.K2_GetActorLocation` _asbp_enemy_rework) "TraceTypeQuery1"))
        (if (not _returnvalue)
          (`/Engine/EditorBlueprintResources/StandardMacros.IsValid` (`self.Objective`)
            (:`Is Valid`
              _)
            (:`Is Not Valid`
              (set `self.Objective` _asbp_enemy_rework)))
          (`SceneComponent.K2_SetWorldRotation` (`self.CanyoGiretori`) (`KismetMathLibrary.MakeRotator` 0.0 (.pitch (`KismetMathLibrary.FindLookAtRotation` (`self.K2_GetActorLocation`) (`self.K2_GetActorLocation` (`self.Objective`)))) (.yaw (`KismetMathLibrary.FindLookAtRotation` (`self.K2_GetActorLocation`) (`self.K2_GetActorLocation` (`self.Objective`))))) false false)
          (if (>= (`self.Seconds Elapsed`) (`/Game/Blueprints/Gameplay/Player/Equipment/Weapon/BP_Item_Weapon.Fire Rate` (`self.Turret Weapon`)))
            (set `self.Seconds Elapsed` 0.0)
            (`/Game/Blueprints/Gameplay/Player/Equipment/Weapon/BP_Item_Weapon.Fire` (`self.Turret Weapon`) (`self.Camera`) false (`self.Bullet Instigator`))
            (break))))
      (else
        (set `PrimitiveComponent.bGenerateOverlapEvents` false (`self.RadiDeVigilancia`))
        (`self.setGadgetState` "NewEnumerator4")
        (set `self.TimeActive` 0.0)
        (set `self.Seconds Elapsed` 0.0)
        (set `self.Objective` (`self.NewObjective`))))
    (elif (`|EnumEquality` _gadgetstate "NewEnumerator4")
      (set `self.TimeActive` (+ (`self.TimeActive`) (`self.Delta Seconds`)))
      (if (not (>= (`self.Cooldown`) (`self.TimeActive`)))
        (`self.setGadgetState` "NewEnumerator1")
        (set `self.TimeActive` 0.0)))))

(fn `Fire`
  (`parent.Fire`)
  (`self.K2_DetachFromActor` "KeepWorld" "KeepWorld" "KeepWorld")
  (`PrimitiveComponent.SetSimulatePhysics` (`self.SkeletalMesh`) true)
  (`self.SetActorTickEnabled` true))

(fn `UserConstructionScript`
  (`parent.UserConstructionScript`)
  (`SphereComponent.SetSphereRadius` (`self.RadiDeVigilancia`) (`self.Turret Radius`) true))