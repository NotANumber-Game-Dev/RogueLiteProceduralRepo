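; Player character Blueprint with axis movement and look, jump, a pause menu, and a three-slot weapon loadout.
; Capsule overlaps notify InteractionInterface actors, and Interact picks up an overlapping weapon into the first free slot, dropping the equipped one when full.
; Fire, reload and slot switching act on the current slot and update the HUD widget.
; UpdateGunAttachments snaps equipped and stowed guns onto separate skeletal mesh components.
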(event `self.ReceiveBeginPlay`
  ;[1 1 1] Show HUD at start
  (bind _returnvalue (`|CreateWidget` "/Game/UI/WBP_HUD.WBP_HUD_C"))
  (bind _output_get (set `self.HUD_Widget` _returnvalue))
  (`UserWidget.AddToViewport` _output_get 0)
  (`WidgetBlueprintLibrary.SetInputMode_GameOnly` (`GameplayStatics.GetPlayerController` 0)))

(event `InputAxis|Foward`
  (params (AxisValue :type "Float (single-precision)"))
  ;[1 1 1] INPUT
  (`self.Movement Foward` AxisValue))

(event `InputAxis|Right`
  (params (AxisValue :type "Float (single-precision)"))
  ;[1 1 1] INPUT
  (`self.Movement Right` AxisValue))

(event `InputAxis|LookUp`
  (params (AxisValue :type "Float (single-precision)"))
  ;[1 1 1] INPUT
  (`self.AddControllerPitchInput` AxisValue))

(event `InputAxis|Turn`
  (params (AxisValue :type "Float (single-precision)"))
  ;[1 1 1] INPUT
  (`self.AddControllerYawInput` AxisValue))

(event `self.CapsuleComponent.OnComponentBeginOverlap`
  (params (OverlappedComponent :type "PrimitiveComponent Object Reference") (OtherActor :type "Actor Object Reference") (OtherComp :type "PrimitiveComponent Object Reference") (OtherBodyIndex :type Integer) (bFromSweep :type Boolean) (SweepResult :type "HitResult Structure (by ref)"))
  ;[1 1 1] Interaction with dropped weapon
  (if (`KismetSystemLibrary.DoesImplementInterface` OtherActor "/Game/Blueprints/Gameplay/Player/InteractionInterface/InteractionInterface.InteractionInterface_C")
    (message `/Game/Blueprints/Gameplay/Player/InteractionInterface/InteractionInterface.OnIteractionRangeEntered` OtherActor self)))

(event `InputAction|Jump`
  (params (Key :type "Key Structure"))
  ;[1 1 1] INPUT
  (:`Pressed`
    (`self.Jump`))
  (:`Released`
    (`self.StopJumping`)))

(event `self.CapsuleComponent.OnComponentEndOverlap`
  (params (OverlappedComponent :type "PrimitiveComponent Object Reference") (OtherActor :type "Actor Object Reference") (OtherComp :type "PrimitiveComponent Object Reference") (OtherBodyIndex :type Integer))
  ;[1 1 1] Interaction with dropped weapon
  (if (`KismetSystemLibrary.DoesImplementInterface` OtherActor "/Game/Blueprints/Gameplay/Player/InteractionInterface/InteractionInterface.InteractionInterface_C")
    (message `/Game/Blueprints/Gameplay/Player/InteractionInterface/InteractionInterface.OnInteractionRangeExited` OtherActor)))

(event `InputAction|Pause Menu`
  (params (Key :type "Key Structure"))
  (bind _returnvalue (`GameplayStatics.GetPlayerController` 0))
  (bind _pause_widget (`self.Pause Widget`))
  ;[1 1 1] INPUT
  (:`Pressed`
    (`/Engine/EditorBlueprintResources/StandardMacros.IsValid` _pause_widget
      (:`Is Valid`
        _)
      (:`Is Not Valid`
        (bind _returnvalue_2 (`|CreateWidget` "/Game/UI/WBP_PauseMenu.WBP_PauseMenu_C"))
        (bind _output_get (set `self.Pause Widget` _returnvalue_2))))
    (set `PlayerController.bShowMouseCursor` true _returnvalue)
    (`WidgetBlueprintLibrary.SetInputMode_UIOnlyEx` _returnvalue _pause_widget)
    (`/Game/UI/WBP_PauseMenu.Show` _output_get)
    (`GameplayStatics.SetGamePaused` true)
    (`/Game/UI/WBP_HUD.Hide HUD` (`self.HUD_Widget`))
    (`/Engine/EditorBlueprintResources/StandardMacros.DoOnce` false
      (:`Completed`
        (`UserWidget.AddToViewport` _output_get 0)))))

(event `InputAction|Interact`
  (params (Key :type "Key Structure"))
  ;[1 1 1] Press F to grab and save item
  (:`Pressed`
    (for _array_element (`PrimitiveComponent.GetOverlappingActors` (`self.CapsuleComponent`) "/Script/Engine.Actor")
      (if (`KismetSystemLibrary.DoesImplementInterface` _array_element "/Game/Blueprints/Gameplay/Player/InteractionInterface/InteractionInterface.InteractionInterface_C")
        (bind _asbp_item_weapon (cast `/Game/Blueprints/Gameplay/Player/Equipment/Weapon/BP_Item_Weapon` _array_element))
        (message `/Game/Blueprints/Gameplay/Player/InteractionInterface/InteractionInterface.OnInteracted` _array_element self)
        (bind _return (`/Game/Blueprints/Gameplay/Player/Equipment/Weapon/BP_Item_Weapon.Get Current Clip Ammo` _asbp_item_weapon))
        (`/Game/UI/WBP_HUD.SetWeapon` (`self.HUD_Widget`) (`self.LastIndexWeponGrabbed`) (`/Game/Blueprints/Gameplay/Player/Equipment/Weapon/BP_Item_Weapon.UI_ShowTexture` _asbp_item_weapon) _return)
        (break)))))

(event `InputAction|Fire`
  (params (Key :type "Key Structure"))
  ;[1 1 1] Shoot
  (:`Pressed`
    (bind _returnvalue (`self.EquippedWeapon`)
      (:`Is Valid`
        (`/Game/Blueprints/Gameplay/Player/Equipment/Weapon/BP_Item_Weapon.Fire` _returnvalue (`self.Camera`))
        (bind _return (`/Game/Blueprints/Gameplay/Player/Equipment/Weapon/BP_Item_Weapon.Get Current Clip Ammo` _returnvalue))
        (`/Game/UI/WBP_HUD.SetAmmoValue` (`self.HUD_Widget`) (`KismetMathLibrary.Conv_ByteToInt` (`self.CurrentWeaponSlot`)) _return)))))

(event `InputAction|Reload`
  (params (Key :type "Key Structure"))
  ;[1 1 1] Reload
  (:`Pressed`
    (bind _returnvalue (`self.EquippedWeapon`)
      (:`Is Valid`
        (`/Game/Blueprints/Gameplay/Player/Equipment/Weapon/BP_Item_Weapon.Reload` _returnvalue)
        (bind _return (`/Game/Blueprints/Gameplay/Player/Equipment/Weapon/BP_Item_Weapon.Get Current Clip Ammo` _returnvalue))
        (`/Game/UI/WBP_HUD.SetAmmoValue` (`self.HUD_Widget`) (`KismetMathLibrary.Conv_ByteToInt` (`self.CurrentWeaponSlot`)) _return)))))

(event `InputAction|SwitchGuns`
  (params (Key :type "Key Structure"))
  (bind _hud_widget (`self.HUD_Widget`))
  ;[1 1 1] TODO: //Rename variables
  (:`Pressed`
    (switch `/Game/Blueprints/Gameplay/Player/Equipment/Weapon/ENUM_Weapon_Slot` (`self.CurrentWeaponSlot`)
      (:`NewEnumerator0`
        (`/Engine/EditorBlueprintResources/StandardMacros.IsValid` (`self.SecondaryGun`)
          (:`Is Valid`
            (set `self.CurrentWeaponSlot` "NewEnumerator1")
            (`/Game/UI/WBP_HUD.SetActiveWeapon` _hud_widget 1))))
      (:`NewEnumerator1`
        (`/Engine/EditorBlueprintResources/StandardMacros.IsValid` (`self.ThirdWeapon`)
          (:`Is Valid`
            (set `self.CurrentWeaponSlot` "NewEnumerator2")
            (`/Game/UI/WBP_HUD.SetActiveWeapon` _hud_widget 2))
          (:`Is Not Valid`
            (set `self.CurrentWeaponSlot` "NewEnumerator0")
            (`/Game/UI/WBP_HUD.SetActiveWeapon` _hud_widget 0))))
      (:`NewEnumerator2`
        (set `self.CurrentWeaponSlot` "NewEnumerator0")
        (`/Game/UI/WBP_HUD.SetActiveWeapon` _hud_widget 0)))
    (`self.Update Gun Attachments`)))

(fn `Combat Reload`)

(fn `Combat Throw Granade`
  (params (index :type Integer)))

(fn `Combat Use Helper`
  (params (index :type Integer)))

(fn `Get Inventory`
  (returns (Inventory :type "/Game/Blueprints/Gameplay/Player/BP_Inventory Object Reference"))
  (return (`self.Inventory`)))

(fn `Movement Crouch`
  (params (value :type Boolean)))

(fn `Movement Foward`
  (params (value :type "Float (double-precision)"))
  (`self.AddMovementInput` (`self.GetActorForwardVector`) value))

(fn `Movement Jump`
  (params (value :type Boolean)))

(fn `Movement Right`
  (params (Value :type "Float (double-precision)"))
  (`self.AddMovementInput` (`self.GetActorRightVector`) Value))

(fn `PickUpGun`
  (params (Weapon :type "/Game/Blueprints/Gameplay/Player/Equipment/Weapon/BP_Item_Weapon Object Reference"))
  (bind _weapon (`local.Weapon`))
  (`/Engine/EditorBlueprintResources/StandardMacros.IsValid` (`self.PrimaryGun`)
    (:`Is Valid`
      (`/Engine/EditorBlueprintResources/StandardMacros.IsValid` (`self.SecondaryGun`)
        (:`Is Valid`
          (`/Engine/EditorBlueprintResources/StandardMacros.IsValid` (`self.ThirdWeapon`)
            (:`Is Valid`
              (bind _returnvalue (`self.EquippedWeapon`)
                (:`Is Valid`
                  (`self.K2_DetachFromActor` _returnvalue "KeepWorld" "KeepWorld" "KeepWorld")
                  (`/Game/Blueprints/Gameplay/Player/Equipment/Weapon/BP_Item_Weapon.Drop` _returnvalue)
                  (`self.SetEquippedWeapon` null)
                  (`self.PickUpGun` (`local.Weapon`)))))
            (:`Is Not Valid`
              (set `self.ThirdWeapon` _weapon)
              (set `self.LastIndexWeponGrabbed` 2)
              (`self.Update Gun Attachments` :!label _label))))
        (:`Is Not Valid`
          (set `self.SecondaryGun` _weapon)
          (set `self.LastIndexWeponGrabbed` 1)
          (goto _label))))
    (:`Is Not Valid`
      (set `self.PrimaryGun` _weapon)
      (set `self.LastIndexWeponGrabbed` 0)
      (goto _label))))

(fn `Update Gun Attachments`
  (bind _primarygun (`self.PrimaryGun`))
  (bind _primarygun_2 (`self.PrimaryGun`))
  (bind _thirdweapon (`self.ThirdWeapon`))
  (bind _primarygun_3 (`self.PrimaryGun`))
  (bind _thirdweapon_2 (`self.ThirdWeapon`))
  (bind _secondarygun (`self.SecondaryGun`))
  (bind _secondarygun_2 (`self.SecondaryGun`))
  (bind _returnvalue (select `/Game/Blueprints/Gameplay/Player/Equipment/Weapon/ENUM_Weapon_Slot` (`self.CurrentWeaponSlot`) :`NewEnumerator0` _primarygun :`NewEnumerator1` (`self.SecondaryGun`) :`NewEnumerator2` (`self.ThirdWeapon`) :!type "Object Object Reference"))
  (`|ExecutionSequence`
    (:`then_0`
      (bind _returnvalue_2 (`self.EquippedWeapon`)
        (:`Is Valid`
          (`self.K2_AttachToComponent` _returnvalue_2 (`self.SkeletalMesh`) "None" "SnapToTarget" "SnapToTarget" "SnapToTarget" true))))
    (:`then_1`
      (if (== _primarygun _returnvalue)
        (`/Engine/EditorBlueprintResources/StandardMacros.IsValid` _secondarygun
          (:`Is Valid`
            (`self.K2_AttachToComponent` _secondarygun (`self.SkeletalMesh1`) "None" "SnapToTarget" "SnapToTarget" "SnapToTarget" true))
          (:`Is Not Valid`
            _))
        (`/Engine/EditorBlueprintResources/StandardMacros.IsValid` _thirdweapon
          (:`Is Valid`
            (`self.K2_AttachToComponent` _thirdweapon (`self.SkeletalMesh2`) "None" "SnapToTarget" "SnapToTarget" "SnapToTarget" true)))
        (elif (== _returnvalue (`self.SecondaryGun`))
          (`/Engine/EditorBlueprintResources/StandardMacros.IsValid` _primarygun_3
            (:`Is Valid`
              (`self.K2_AttachToComponent` _primarygun_3 (`self.SkeletalMesh1`) "None" "SnapToTarget" "SnapToTarget" "SnapToTarget" true))
            (:`Is Not Valid`
              _))
          (`/Engine/EditorBlueprintResources/StandardMacros.IsValid` _thirdweapon_2
            (:`Is Valid`
              (`self.K2_AttachToComponent` _thirdweapon_2 (`self.SkeletalMesh2`) "None" "SnapToTarget" "SnapToTarget" "SnapToTarget" true)))
          (else
            (`/Engine/EditorBlueprintResources/StandardMacros.IsValid` _primarygun_2
              (:`Is Valid`
                (`self.K2_AttachToComponent` _primarygun_2 (`self.SkeletalMesh1`) "None" "SnapToTarget" "SnapToTarget" "SnapToTarget" true))
              (:`Is Not Valid`
                _))
            (`/Engine/EditorBlueprintResources/StandardMacros.IsValid` _secondarygun_2
              (:`Is Valid`
                (`self.K2_AttachToComponent` _secondarygun_2 (`self.SkeletalMesh2`) "None" "SnapToTarget" "SnapToTarget" "SnapToTarget" true)))))))))

(fn `UserConstructionScript`
  (bind _returnvalue (`|GenericCreateObject` "/Game/Blueprints/Gameplay/Player/BP_Inventory.BP_Inventory_C" (`self.Inventory`)))
  (set `self.Inventory` _returnvalue))