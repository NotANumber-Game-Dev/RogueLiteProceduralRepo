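; Enemy helper that picks a cover location hidden from the player and reports when none qualifies.
; FindCoverPoints line-traces inward from a ring around the player's navmesh-projected position, storing blocking hits pushed out along their normals.
; LocationToHide filters these by minimum player distance and enemy radius, then keeps the last within Closest, which is never updated.
; Only the point set is cleared between calls, not the filtered arrays.
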(fn `FindCoverPoints`
  (returns (LocationsToCover :type "Array of Vector Structure"))
  (bind _projectedlocation (`NavigationSystemV1.K2_ProjectPointToNavigation` (`Actor.K2_GetActorLocation` (`GameplayStatics.GetPlayerCharacter` 0)) null "/Script/NavigationSystem.RecastFilter_UseDefaultArea"))
  (bind _returnvalue (`KismetMathLibrary.MakeVector` (.x _projectedlocation) (.y _projectedlocation) (+ (.z _projectedlocation) 50.0)))
  (`KismetArrayLibrary.Array_Clear` (`self.LocationSet`))
  ;[1 1 1] Mirarem al voltant del enemy amb una precicio de 10 graus
  (for _index (range 71)
    (bind (_outhit _returnvalue_2) (`KismetSystemLibrary.LineTraceSingle` (+ (* (`KismetMathLibrary.GreaterGreater_VectorRotator` (1.0 0.0 0.0) (`KismetMathLibrary.MakeRotator` 0.0 0.0 (* _index 5.0))) (`self.RadiusToCheck`)) _returnvalue) _returnvalue "TraceTypeQuery1"))
    (if _returnvalue_2
      (bind (_bblockinghit _binitialoverlap _time _distance _location _impactpoint _normal _impactnormal) (`GameplayStatics.BreakHitResult` _outhit))
      (`KismetArrayLibrary.Array_Add` (`self.LocationSet`) (+ _impactpoint (* _impactnormal 200.0)))))
  (return (`self.LocationSet`)))

(fn `LocationToHide`
  (params (EnemyPos :type "Vector Structure"))
  (returns (ClosestCover :type "Vector Structure") (isNull :type Boolean))
  (locals (finalLocation :type "Vector Structure") (closest :type "Float (double-precision)" :default 10000000000.0) (LocationsAwayFromPlayer :type "Array of Vector Structure") (isNullArray :type Boolean :default false) (`Enemy Position` :type "Vector Structure") (LocationsCloseToEnemy :type "Array of Vector Structure"))
  (set `local.Enemy Position` EnemyPos)
  (bind _locationstocover (`self.FindCoverPoints`))
  (for _array_element _locationstocover
    (if (>= (`KismetMathLibrary.Vector_Distance2D` _array_element (`Actor.K2_GetActorLocation` (`GameplayStatics.GetPlayerCharacter` 0))) (`self.RangeFromPlayer`))
      (`KismetArrayLibrary.Array_Add` (`local.LocationsAwayFromPlayer`) _array_element)))
  (if (!= (`KismetArrayLibrary.Array_Length` (`local.LocationsAwayFromPlayer`)) 0)
    (set `local.isNullArray` false)
    (for _array_element_2 (`local.LocationsAwayFromPlayer`)
      (if (<= (`KismetMathLibrary.Vector_Distance2D` _array_element_2 (`local.Enemy Position`)) (`self.RadiusFromEnemy`))
        (`KismetArrayLibrary.Array_Add` (`local.LocationsCloseToEnemy`) _array_element_2)))
    (if (!= (`KismetArrayLibrary.Array_Length` (`local.LocationsCloseToEnemy`)) 0)
      (set `local.isNullArray` false)
      (for _array_element_3 (`local.LocationsCloseToEnemy`)
        (if (<= (`KismetMathLibrary.Vector_Distance2D` _array_element_3 (`local.Enemy Position`)) (`local.closest`))
          (set `local.finalLocation` _array_element_3)))
      (return (`local.finalLocation`) (`local.isNullArray`))
      (else
        (set `local.isNullArray` true)))
    (else
      (set `local.isNullArray` true))))