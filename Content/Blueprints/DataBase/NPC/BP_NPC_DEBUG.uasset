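; BP_NPC_DEBUG is a debug NPC Blueprint that adds quest handling to its parent's UI-related action.
; Its ExecUIRelated override runs the parent logic, then branches on GetSetNextQuest, which is commented as a null-pointer guard.
; A true result goes straight to ENDING, while a false one first sets the quest state to Grabbed and calls SetCounterForEnemiesKilled.
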(fn `ExecUIRelated`
  (`parent.ExecUIRelated`)
  (bind _no_more_quests (`self.Get Set Next Quest`))
  ;[1 1 1] Check not to go in null pointer
  (if _no_more_quests
    (`self.ENDING`)
    (else
      (`self.Set Quest State` "Grabbed")
      (`self.Set Counter For Enemies Killed`)
      (`self.ENDING`))))

(fn `UserConstructionScript`
  (`parent.UserConstructionScript`))