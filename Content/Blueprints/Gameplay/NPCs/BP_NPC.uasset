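; Quest-giving NPC that shows an interaction tooltip, turns toward a nearby player and opens a paged dialogue widget.
; On interaction it locks player movement and camera, then loads the current quest's lines from the game instance's quest database by NPC class.
; Advance pages through the lines, then calls the empty ExecUIRelated hook.
; Helper functions update quest state and counters; ENDING restores player control and HUD.
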(event `/Game/Blueprints/Gameplay/Player/InteractionInterface/InteractionInterface.OnIteractionRangeEntered`
  (params (Player :type "/Game/Blueprints/Gameplay/Player/BP_Player Object Reference"))
  (bind _hud_widget (`/Game/Blueprints/Gameplay/Player/BP_Player.HUD_Widget` Player))
  (`/Game/UI/WBP_HUD.Set Tooltip` _hud_widget (`KismetTextLibrary.Conv_StringToText` (`KismetStringLibrary.Concat_StrStr` (`KismetStringLibrary.Concat_StrStr` (`KismetTextLibrary.Conv_TextToString` (`self.InteractionToolTip`)) " ") (`KismetTextLibrary.Conv_TextToString` (`self.Name`)))) true)
  (`/Game/UI/WBP_HUD.Show Tooltip` _hud_widget))

(event `/Game/Blueprints/Gameplay/Player/InteractionInterface/InteractionInterface.OnInteractionRangeExited`
  (`/Game/UI/WBP_HUD.Hide Tooltip` (`/Game/Blueprints/Gameplay/Player/BP_Player.HUD_Widget` (stale `/Game/Blueprints/Gameplay/Player/InteractionInterface/InteractionInterface.OnIteractionRangeEntered` Player))))

(event `Should Rotate`
  ;[1 1 1] Should Rotate
  (if (<= (`self.GetDistanceTo` (`self.Char REF`)) (`self.Distance To Rotate`))
    (set `self.Should Rotate to Player` true)
    (`self.Face Player`)
    (else
      (set `self.Should Rotate to Player` false)))
  (`KismetSystemLibrary.Delay` 0.001)
  (`self.Should Rotate`))

(event `Face Player`
  (bind (_returnvalue_roll _returnvalue_pitch _returnvalue_yaw) (`KismetMathLibrary.BreakRotator` (`KismetMathLibrary.RInterpTo` (`self.K2_GetActorRotation`) (`KismetMathLibrary.FindLookAtRotation` (`self.K2_GetActorLocation`) (`self.K2_GetActorLocation` (`self.Char REF`))) (`GameplayStatics.GetWorldDeltaSeconds`) 5.0)))
  ;[1 1 1] Face player
  (if (`self.Should Rotate to Player`)
    (`self.K2_SetActorRotation` (`KismetMathLibrary.MakeRotator` 0.0 0.0 _returnvalue_yaw))
    (`KismetSystemLibrary.Delay` 0.001)
    (`self.Face Player`)
    (else
      (`self.Should Rotate`))))

(event `self.ReceiveBeginPlay`
  (bind _asbp_controlled_main_game_instance (cast `/Game/Blueprints/GameModes/BP_ControlledMainGameInstance` (`GameplayStatics.GetGameInstance`)))
  (set `self.GAME INSTANCE` _asbp_controlled_main_game_instance)
  (bind _returnvalue (`|CreateWidget` "/Game/UI/WBP_Dialogue.WBP_Dialogue_C"))
  (bind _output_get (set `self.Dialog` _returnvalue))
  (`/Game/UI/WBP_Dialogue.Set Owning NPC` _output_get self)
  (bind _asbp_player (cast `/Game/Blueprints/Gameplay/Player/BP_Player` (`GameplayStatics.GetPlayerCharacter` 0)))
  (set `self.Char REF` _asbp_player)
  (`self.Should Rotate`))

(event `/Game/Blueprints/Gameplay/Player/InteractionInterface/InteractionInterface.OnInteracted`
  (params (Player :type "/Game/Blueprints/Gameplay/Player/BP_Player Object Reference"))
  (if (not (`self.IsInDialog`))
    (set `self.IsInDialog` true)
    (`self.Get Set Next Quest`)
    (`self.Get Paragraphs for Quest`)
    (set `self.currentDialog` 0)
    (`|ExecutionSequence`
      (:`then_0`
        (`self.SetNameNPC` (`KismetTextLibrary.Conv_TextToString` (`self.Name`)))
        (`self.SetParagraphNPC` (`|GetArrayItem` (`self.Paragraph`) (`self.currentDialog`)))
        (`KismetSystemLibrary.PrintString` "Hello"))
      (:`then_1`
        (`UserWidget.AddToViewport` (`self.Dialog`) 0)
        (bind _asbp_player (cast `/Game/Blueprints/Gameplay/Player/BP_Player` (`GameplayStatics.GetPlayerPawn` 0)))
        (set `/Game/Blueprints/Gameplay/Player/BP_Player.canRotateCamara` false _asbp_player)
        (set `/Game/Blueprints/Gameplay/Player/BP_Player.Can move` false _asbp_player)))))

(event `self.ReceiveTick`
  (params (DeltaSeconds :type "Float (single-precision)"))
  (bind _sphere (`self.Sphere`))
  (if (`self.IsInDialog`)
    (`ActorComponent.Deactivate` _sphere)
    (else
      (`ActorComponent.SetActive` _sphere true false))))

(fn `Add Enemies Killed Cunter`
  (`DATABASE.AddEnemiesKilledCounter` (`/Game/Blueprints/GameModes/BP_ControlledMainGameInstance.DATABASE` (`self.GAME INSTANCE`))))

(fn `Advance`
  (if (`self.IsInDialog`)
    (bind _output_get (set `self.currentDialog` (+ (`self.currentDialog`) 1)))
    (if (> _output_get (- (`KismetArrayLibrary.Array_Length` (`self.Paragraph`)) 1))
      (`self.ExecUIRelated`)
      (`Widget.RemoveFromParent` (`self.Dialog`))
      (set `self.IsInDialog` false)
      (else
        (`self.SetParagraphNPC` (`|GetArrayItem` (`self.Paragraph`) (`self.currentDialog`)))))))

(fn `ENDING`
  (bind _returnvalue (`GameplayStatics.GetPlayerController` 0))
  (`GameplayStatics.SetGamePaused` false)
  (set `PlayerController.bShowMouseCursor` false _returnvalue)
  (`WidgetBlueprintLibrary.SetInputMode_GameOnly` _returnvalue)
  (bind _asbp_player (cast `/Game/Blueprints/Gameplay/Player/BP_Player` (`GameplayStatics.GetPlayerPawn` 0)))
  (set `/Game/Blueprints/Gameplay/Player/BP_Player.canRotateCamara` true _asbp_player)
  (set `/Game/Blueprints/Gameplay/Player/BP_Player.Can move` true _asbp_player)
  (`UserWidget.AddToViewport` (`/Game/Blueprints/Gameplay/Player/BP_Player.HUD_Widget` _asbp_player) 0))

(fn `ExecUIRelated`)

(fn `Get Paragraphs for Quest`
  (for _array_element (`DATABASE.DATABASE_QUEST_LIST` (`/Game/Blueprints/GameModes/BP_ControlledMainGameInstance.DATABASE` (`self.GAME INSTANCE`)))
    (if (== (break `NPC_Quest_List` _array_element) (`GameplayStatics.GetObjectClass` self))
      (`KismetSystemLibrary.PrintString` (`KismetStringLibrary.Conv_IntToString` (`.Mission_Index` (break `NPC_Quest_List` _array_element))))
      (`KismetArrayLibrary.Array_Clear` (`self.Paragraph`))
      (for _array_element_2 (`.NPC_Dialogues` (break `Quest` (`|GetArrayItem` (`.Quest_List` (break `NPC_Quest_List` _array_element)) (`.Mission_Index` (break `NPC_Quest_List` _array_element)))))
        (`KismetArrayLibrary.Array_Add` (`self.Paragraph`) (`KismetTextLibrary.Conv_TextToString` _array_element_2))))))

(fn `Get Set Next Quest`
  (returns (`No More quests` :type Boolean))
  (bind _nomoremisions (`DATABASE.GetNextQuest` (`/Game/Blueprints/GameModes/BP_ControlledMainGameInstance.DATABASE` (`self.GAME INSTANCE`)) (`GameplayStatics.GetObjectClass` self)))
  (return _nomoremisions))

(fn `Set Counter For Enemies Killed`
  (`DATABASE.SetCounterForEnemiesKilled` (`/Game/Blueprints/GameModes/BP_ControlledMainGameInstance.DATABASE` (`self.GAME INSTANCE`)) (`GameplayStatics.GetObjectClass` self) (`self.QUEST_INDEX`) 0))

(fn `Set Counter For Interact With Item`
  (`DATABASE.SetCounterForInteractWithItem` (`/Game/Blueprints/GameModes/BP_ControlledMainGameInstance.DATABASE` (`self.GAME INSTANCE`)) (`GameplayStatics.GetObjectClass` self) (`self.QUEST_INDEX`) false))

(fn `Set Counter For Recollection Items`
  (`DATABASE.SetCounterForRecolectionItems` (`/Game/Blueprints/GameModes/BP_ControlledMainGameInstance.DATABASE` (`self.GAME INSTANCE`)) (`GameplayStatics.GetObjectClass` self) (`self.QUEST_INDEX`) 0))

(fn `Set Counter Kill Specific Enemy`
  (`DATABASE.SetCounterForKillSpecificEnemy` (`/Game/Blueprints/GameModes/BP_ControlledMainGameInstance.DATABASE` (`self.GAME INSTANCE`)) (`GameplayStatics.GetObjectClass` self) (`self.QUEST_INDEX`) 0))

(fn `Set Counter N Specific Enemy`
  (`DATABASE.SetCounterNSpecificEnemiesKilled` (`/Game/Blueprints/GameModes/BP_ControlledMainGameInstance.DATABASE` (`self.GAME INSTANCE`)) (`GameplayStatics.GetObjectClass` self) (`self.QUEST_INDEX`) 0))

(fn `Set Quest State`
  (params (inState :type "EQuest_State Enum" :default "Not_Grabbed"))
  (`DATABASE.SetStateQuest` (`/Game/Blueprints/GameModes/BP_ControlledMainGameInstance.DATABASE` (`self.GAME INSTANCE`)) (`GameplayStatics.GetObjectClass` self) (`self.QUEST_INDEX`) inState))

(fn `SetNameNPC`
  (params (name :type String))
  (`/Game/UI/WBP_Dialogue.Set Name` (`self.Dialog`) (`KismetTextLibrary.Conv_StringToText` name)))

(fn `SetParagraphNPC`
  (params (Paragraph :type String))
  (`/Game/UI/WBP_Dialogue.Set Paragraph` (`self.Dialog`) (`KismetTextLibrary.Conv_StringToText` Paragraph)))

(fn `UserConstructionScript`)