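; BP_RandomMesh is a prop that shows a random material on its Plane component; despite the name, it swaps no meshes.
; The construction script and BeginPlay each pick independently from MeshesToShown and set material slot 0, so the in-game look can differ from the construction-time one.
; The random range's inclusive maximum is the array length, so the index can land one past the last entry.
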(event `self.ReceiveBeginPlay`
  (bind _output_materialinterface (break `StaticMaterial` (`|GetArrayItem` (`self.MeshesToShown`) (`KismetMathLibrary.RandomIntegerInRange` 0 (`KismetArrayLibrary.Array_Length` (`self.MeshesToShown`))))))
  (`PrimitiveComponent.SetMaterial` (`self.Plane`) 0 _output_materialinterface))

(fn `UserConstructionScript`
  (bind _output_materialinterface (break `StaticMaterial` (`|GetArrayItem` (`self.MeshesToShown`) (`KismetMathLibrary.RandomIntegerInRange` 0 (`KismetArrayLibrary.Array_Length` (`self.MeshesToShown`))))))
  (`PrimitiveComponent.SetMaterial` (`self.Plane`) 0 _output_materialinterface))