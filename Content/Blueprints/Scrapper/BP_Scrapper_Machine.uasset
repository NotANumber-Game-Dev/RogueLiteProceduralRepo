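; BP_Scrapper_Machine is an interactable scrapper machine that opens the scrapper UI.
; It creates a WBP_Scrapper widget on BeginPlay and keeps it for reuse.
; On interaction, a DoOnce adds the widget to the viewport the first time, and every interaction shows it, pauses the game, and switches to UI-only input with the mouse cursor visible.
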(event `self.ReceiveBeginPlay`
  (bind _returnvalue (`|CreateWidget` "/Game/UI/Components/Scrapper_Oriol/WBP_Scrapper.WBP_Scrapper_C"))
  (set `self.Scraper_Widget` _returnvalue))

(event `self.ReceiveActorBeginOverlap`
  (params (OtherActor :type "Actor Object Reference")))

(event `/Game/Blueprints/Gameplay/Player/InteractionInterface/InteractionInterface.OnInteracted`
  (params (Player :type "/Game/Blueprints/Gameplay/Player/BP_Player Object Reference"))
  (bind _returnvalue (`GameplayStatics.GetPlayerController` 0))
  (bind _scraper_widget (`self.Scraper_Widget`))
  (`|ExecutionSequence`
    (:`then_0`
      (`/Engine/EditorBlueprintResources/StandardMacros.DoOnce` false
        (:`Completed`
          (`UserWidget.AddToViewport` _scraper_widget 0))))
    (:`then_1`
      (`/Game/UI/Components/Scrapper_Oriol/WBP_Scrapper.Show` _scraper_widget)
      (`GameplayStatics.SetGamePaused` true)
      (`WidgetBlueprintLibrary.SetInputMode_UIOnlyEx` _returnvalue null)
      (set `PlayerController.bShowMouseCursor` true _returnvalue))))

(fn `UserConstructionScript`)