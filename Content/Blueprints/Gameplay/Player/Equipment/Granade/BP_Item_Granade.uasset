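; BP_Item_Granade is a grenade item the player picks up by interacting, then equips, stores and fires.
; SetGranadeState switches between Dropped with physics and overlap, Equipped as hidden and attached to player 0's EnMano component, and Stored as hidden without collision.
; Fire decrements ammo and spawns a BP_GranadeProjectile launched toward a point along the camera's forward vector, passing type and explosion range.
; IsSameGrande compares two grenades by type.
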(event `self.ReceiveBeginPlay`
  (`self.setGranadeState` "NewEnumerator0"))

(event `/Game/Blueprints/Gameplay/Player/InteractionInterface/InteractionInterface.OnInteracted`
  (params (Player :type "/Game/Blueprints/Gameplay/Player/BP_Player Object Reference"))
  (`/Game/Blueprints/Gameplay/Player/BP_Player.PickUpGranade` Player self))

(fn `Fire`
  (params (FiredGranade :type "/Game/Blueprints/Gameplay/Player/Equipment/Granade/BP_Item_Granade Object Reference") (PlayerCamera :type "CameraComponent Object Reference"))
  (locals (NewLocalVar_0 :type "Transform Structure"))
  (bind _result (`/Engine/EditorBlueprintResources/StandardMacros.DecrementInt` (`self.Ammo`))
    (:`  `
      (set `self.Ammo` _result)
      (`|SpawnActorFromClass` "/Game/Blueprints/Gameplay/Player/Equipment/Granade/BP_GranadeProjectile.BP_GranadeProjectile_C" (`KismetMathLibrary.MakeTransform` (`self.K2_GetActorLocation`)) "Undefined" "OverrideRootScale" null (`/Game/Blueprints/Gameplay/Player/Equipment/Granade/BP_Item_Granade.Type` FiredGranade) (* (`KismetMathLibrary.Normal` (- (+ (`SceneComponent.K2_GetComponentLocation` PlayerCamera) (* (`SceneComponent.GetForwardVector` PlayerCamera) (`self.GranadeRange`))) (`SceneComponent.GetSocketLocation` (`self.SkeletalMesh`) "None"))) (* (`self.GranadeVelocity`) 1000.0)) (`self.RadiExplosio`) null))))

(fn `HideMesh`
  (`SceneComponent.SetVisibility` (`self.SkeletalMesh`) false true))

(fn `isSameGrande`
  (params (NewGranade :type "/Game/Blueprints/Gameplay/Player/Equipment/Granade/BP_Item_Granade Object Reference") (CurrentGranadeSlotToCheck :type "/Game/Blueprints/Gameplay/Player/Equipment/Granade/BP_Item_Granade Object Reference"))
  (returns (ReturnValue :type Boolean))
  (return (`|EnumEquality` (`/Game/Blueprints/Gameplay/Player/Equipment/Granade/BP_Item_Granade.Type` NewGranade) (`/Game/Blueprints/Gameplay/Player/Equipment/Granade/BP_Item_Granade.Type` CurrentGranadeSlotToCheck))))

(fn `setGranadeState`
  (params (`New State` :type "/Game/Blueprints/Gameplay/Player/Equipment/Granade/ENUM_GranadeStates Enum" :default "NewEnumerator0"))
  (bind _sphere (`self.Sphere`))
  (bind _skeletalmesh (`self.SkeletalMesh`))
  (bind _skeletalmesh_2 (`self.SkeletalMesh`))
  (bind _output_get (set `self.GranadeState` `New State`))
  (switch `/Game/Blueprints/Gameplay/Player/Equipment/Granade/ENUM_GranadeStates` _output_get
    (:`NewEnumerator0`
      (`PrimitiveComponent.SetCollisionProfileName` _sphere "OverlapAllDynamic" true)
      (`PrimitiveComponent.SetSimulatePhysics` _skeletalmesh_2 true)
      (`PrimitiveComponent.SetCollisionProfileName` _skeletalmesh_2 "DroppedWeapon" true))
    (:`NewEnumerator1`
      (`self.SetActorTickEnabled` false)
      (`PrimitiveComponent.SetCollisionEnabled` _sphere "NoCollision")
      (`PrimitiveComponent.SetSimulatePhysics` _skeletalmesh_2 false)
      (`PrimitiveComponent.SetCollisionEnabled` _skeletalmesh_2 "NoCollision")
      (`SceneComponent.ResetRelativeTransform` _skeletalmesh_2)
      (`self.hideMesh`)
      (bind _asbp_player (cast `/Game/Blueprints/Gameplay/Player/BP_Player` (`GameplayStatics.GetPlayerPawn` 0)))
      (`self.K2_AttachToComponent` (`/Game/Blueprints/Gameplay/Player/BP_Player.EnMano` _asbp_player) "None" "SnapToTarget" "SnapToTarget" "SnapToTarget"))
    (:`NewEnumerator2`
      (`self.SetActorTickEnabled` false)
      (`PrimitiveComponent.SetCollisionEnabled` (`self.Sphere`) "NoCollision")
      (`PrimitiveComponent.SetSimulatePhysics` _skeletalmesh false)
      (`PrimitiveComponent.SetCollisionEnabled` _skeletalmesh "NoCollision")
      (`SceneComponent.ResetRelativeTransform` _skeletalmesh)
      (`self.hideMesh`))))

(fn `ShowMesh`
  (`SceneComponent.SetVisibility` (`self.SkeletalMesh`) true true))

(fn `UserConstructionScript`
  (`parent.UserConstructionScript`))