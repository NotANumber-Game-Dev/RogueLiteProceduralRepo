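; Weapon item actor that can be picked up, equipped and dropped, switching physics and collision with each state.
; Fire spawns velocity-driven bullets with random spread, muzzle flash and sound, for players and non-players.
; Player recoil plays a timeline into controller input, then reverses it on stop, scaling pitch recovery by aim drift for certain weapon types.
; Reload draws on reserve ammo with HUD tooltips for players; non-players refill freely.
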(event `self.ReceiveTick`
  (params (DeltaSeconds :type "Float (single-precision)")))

(event `/Game/Blueprints/Gameplay/Player/InteractionInterface/InteractionInterface.OnInteracted`
  (params (Player :type "/Game/Blueprints/Gameplay/Player/BP_Player Object Reference"))
  (`/Game/Blueprints/Gameplay/Player/BP_Player.PickUpGun` Player self)
  (`self.setWeaponState` "NewEnumerator1")
  ;[1 1 1] missio
  (`self.AddItemToMission`))

(event `self.ReceiveBeginPlay`
  (`self.setWeaponState` "NewEnumerator0")
  (bind _returnvalue (`|CreateWidget` "/Game/UI/Components/Game/Inventory/WBP_Inventory_Item.WBP_Inventory_Item_C"))
  (bind _output_get (set `self.Inventory UI` _returnvalue))
  (`/Game/UI/Components/Game/Inventory/WBP_Inventory_Item.Set Image` _output_get (`self.UI_ShowTexture`)))

(event `RecoilOnFire`
  (bind _recoilmaxthreshold (`self.RecoilMaxThreshold`))
  (bind _returnvalue (`KismetMathLibrary.Abs` (.pitch (`KismetMathLibrary.NormalizedDeltaRotator` (`self.OriginRotation`) (`self.PostRecoilRotation`)))))
  (if (and (`|EnumInequality` (`self.type`) "NewEnumerator0") (`|EnumInequality` (`self.type`) "NewEnumerator3"))
    (`TimelineComponent.SetPlayRate` (`self.RecoilTimepline`) 1.0)
    (`|ExecutionSequence`
      (:`then_0`
        (`/Engine/EditorBlueprintResources/StandardMacros.DoOnce` false :!label _label
          (:`Completed`
            (set `self.OriginRotation` (`Controller.GetControlRotation` (`GameplayStatics.GetPlayerController` 0))))))
      (:`then_1`
        (bind (_direction _pitchinput _yawinput) (`Timeline|RecoilTimepline` :!label _label_2)
          (:`Update`
            (`KismetSystemLibrary.PrintString` (`KismetStringLibrary.Conv_DoubleToString` (.pitch (`KismetMathLibrary.NormalizedDeltaRotator` (`self.OriginRotation`)))) false false)
            (switch `ETimelineDirection` _direction
              (:`Forward`
                (`self.Update Recoil Pos` _pitchinput _yawinput))
              (:`Backward`
                (`|ExecutionSequence`
                  (:`then_0`
                    (`/Engine/EditorBlueprintResources/StandardMacros.DoOnce` false :!label _label_3
                      (:`Completed`
                        (set `self.PostRecoilRotation` (`Controller.GetControlRotation` (`GameplayStatics.GetPlayerController` 0))))))
                  (:`then_1`
                    (`self.Update Recoil Pos` (* _pitchinput -13.0 (select `bool` (> _returnvalue _recoilmaxthreshold) :`false` (`KismetMathLibrary.MapRangeClamped` _returnvalue 0.0 _recoilmaxthreshold 0.0 1.0) :`true` (`KismetMathLibrary.MapRangeClamped` _returnvalue _recoilmaxthreshold 30.0 1.0)))))))))
          (:`Finished`
            (switch `ETimelineDirection` _direction
              (:`Backward`
                (`self.RecoilReset`)))))))
    (else
      (`KismetSystemLibrary.PrintString` "No Recoil Weaopn" false false :!label _label_4)
      (goto _label_2 :!via `Stop`))))

(event `RecoilStopFire`
  (if (and (`|EnumInequality` (`self.type`) "NewEnumerator0") (`|EnumInequality` (`self.type`) "NewEnumerator3"))
    (`TimelineComponent.SetPlayRate` (`self.RecoilTimepline`) 13.0)
    (goto _label_2 :!via `Reverse`)
    (else
      (goto _label_4))))

(event `RecoilReset`
  (if (and (`|EnumInequality` (`self.type`) "NewEnumerator0") (`|EnumInequality` (`self.type`) "NewEnumerator3"))
    (`|ExecutionSequence`
      (:`then_0`
        (goto _label :!via `Reset`))
      (:`then_1`
        (goto _label_3 :!via `Reset`)))
    (else
      (goto _label_4))))

(fn `Drop`
  (`self.setWeaponState` "NewEnumerator0"))

(fn `Fire`
  (params (`Player Camera` :type "CameraComponent Object Reference") (isPlayer :type Boolean) (WhoShoted :type "Pawn Object Reference"))
  (returns (NeedsReload :type Boolean) (HasShooted :type Boolean))
  (bind _returnvalue (`SceneComponent.K2_GetComponentLocation` `Player Camera`))
  (bind _returnvalue_2 (`self.K2_GetActorRotation`))
  (bind _returnvalue_3 (`SceneComponent.GetSocketLocation` (`self.SkeletalMesh`) "b_gun_muzzleflash"))
  (bind _returnvalue_4 (* (`self.Bullet Velocity`) 1000.0))
  (if (> (`self.Current Clip`) 0)
    (set `self.Current Clip` (- (`self.Current Clip`) 1))
    (if isPlayer
      (`|SpawnActorFromClass` "/Game/Blueprints/Gameplay/Player/Equipment/Bullet/BP_Bullet.BP_Bullet_C" (`KismetMathLibrary.MakeTransform` _returnvalue_3 (`self.K2_GetActorRotation`)) "Undefined" "OverrideRootScale" null (* (`KismetMathLibrary.Normal` (- (+ _returnvalue (* (`self.Spread Trace` (`SceneComponent.GetForwardVector` `Player Camera`)) (`self.Bullet Range`))) _returnvalue_3)) _returnvalue_4) (`self.ExplosiveBullets`) WhoShoted)
      (if (not (`|EnumEquality` (`self.type`) "NewEnumerator4"))
        (bind _returnvalue_5 (`|SpawnActorFromClass` "/Game/Blueprints/Gameplay/Player/Equipment/Bullet/BP_ShootFlash.BP_ShootFlash_C" (`KismetMathLibrary.MakeTransform` _returnvalue_3 _returnvalue_2) "Undefined" "OverrideRootScale" null null))
        (`SceneComponent.K2_AttachToComponent` (`/Game/Blueprints/Gameplay/Player/Equipment/Bullet/BP_ShootFlash.Arrow` _returnvalue_5) (`self.SkeletalMesh`) "b_gun_muzzleflash" "SnapToTarget" "KeepWorld" "SnapToTarget" true)
        (`self.RecoilOnFire`)
        (bind _returnvalue_6 (`GameplayStatics.SpawnSoundAtLocation` (`self.Fire_Sound`) (`self.K2_GetActorLocation`) (struct) 1.0 1.0 0.0 null null :!label _label))
        (`AudioComponent.Play` _returnvalue_6 0.0)
        (return false true))
      (else
        (`|SpawnActorFromClass` "/Game/Blueprints/Gameplay/Player/Equipment/Bullet/BP_Bullet.BP_Bullet_C" (`KismetMathLibrary.MakeTransform` _returnvalue_3 (`self.K2_GetActorRotation`)) "Undefined" "OverrideRootScale" null (`self.Spread Trace` (* (`KismetMathLibrary.Normal` (- (+ _returnvalue (* (`SceneComponent.GetForwardVector` `Player Camera`) (`self.Bullet Range`))) _returnvalue_3)) _returnvalue_4)) false WhoShoted)
        (if (not (`|EnumEquality` (`self.type`) "NewEnumerator4"))
          (bind _returnvalue_7 (`|SpawnActorFromClass` "/Game/Blueprints/Gameplay/Player/Equipment/Bullet/BP_ShootFlash.BP_ShootFlash_C" (`KismetMathLibrary.MakeTransform` _returnvalue_3 _returnvalue_2) "Undefined" "OverrideRootScale" null null))
          (`SceneComponent.K2_AttachToComponent` (`/Game/Blueprints/Gameplay/Player/Equipment/Bullet/BP_ShootFlash.Arrow` _returnvalue_7) (`self.SkeletalMesh`) "b_gun_muzzleflash" "SnapToTarget" "KeepWorld" "SnapToTarget" true)
          (goto _label))))
    (elif isPlayer
      (bind _asbp_player (cast `/Game/Blueprints/Gameplay/Player/BP_Player` (`GameplayStatics.GetPlayerPawn` 0)))
      (bind _hud_widget (`/Game/Blueprints/Gameplay/Player/BP_Player.HUD_Widget` _asbp_player))
      (`/Game/UI/WBP_HUD.Set Tooltip` _hud_widget "Need To Realod!" false)
      (`/Game/UI/WBP_HUD.Show Tooltip` _hud_widget)
      (`self.RecoilStopFire`)
      (return true false))))

(fn `Get Current Ammo`
  (returns (`Current Total Ammo` :type Integer))
  (return (`self.Current Total Ammo`)))

(fn `Get Current Clip Ammo`
  (returns (return :type Integer))
  (return (`self.Current Clip`)))

(fn `getInteractionTextAttached`
  (returns (AttachedComponent :type "SceneComponent Object Reference"))
  (return (`self.SkeletalMesh`)))

(fn `Hide Mesh`
  (`SceneComponent.SetVisibility` (`self.SkeletalMesh`) false true))

(fn `Reload`
  (params (isPlayer :type Boolean))
  (bind _clip_size (`self.Clip Size`))
  (bind _returnvalue (- (`self.Current Total Ammo`) _clip_size))
  (if isPlayer
    (if (>= _returnvalue 0)
      (set `self.Current Total Ammo` _returnvalue)
      (set `self.Current Clip` _clip_size)
      (bind _asbp_player (cast `/Game/Blueprints/Gameplay/Player/BP_Player` (`GameplayStatics.GetPlayerPawn` 0)))
      (bind _hud_widget (`/Game/Blueprints/Gameplay/Player/BP_Player.HUD_Widget` _asbp_player))
      (`/Game/UI/WBP_HUD.Set Tooltip` _hud_widget "" false)
      (`/Game/UI/WBP_HUD.Show Tooltip` _hud_widget)
      (else
        (bind _asbp_player_2 (cast `/Game/Blueprints/Gameplay/Player/BP_Player` (`GameplayStatics.GetPlayerPawn` 0)))
        (bind _hud_widget_2 (`/Game/Blueprints/Gameplay/Player/BP_Player.HUD_Widget` _asbp_player_2))
        (`/Game/UI/WBP_HUD.Set Tooltip` _hud_widget_2 "Out Of Bullets!" false)
        (`/Game/UI/WBP_HUD.Show Tooltip` _hud_widget_2)))
    (else
      (set `self.Current Clip` _clip_size))))

(fn `SetSkeletalMesh`
  (params (NewSkeletalMesh :type "SkeletalMesh Object Reference"))
  (bind _skeletalmesh (`self.SkeletalMesh`))
  (`/Engine/EditorBlueprintResources/StandardMacros.IsValid` NewSkeletalMesh
    (:`Is Valid`
      (`SkinnedMeshComponent.SetSkinnedAssetAndUpdate` _skeletalmesh NewSkeletalMesh true))
    (:`Is Not Valid`
      (`SkinnedMeshComponent.SetSkinnedAssetAndUpdate` _skeletalmesh "/Engine/EngineMeshes/SkeletalCube.SkeletalCube" true))))

(fn `setWeaponState`
  (params (`New WeaponState` :type "/Game/Blueprints/Gameplay/Player/Equipment/Weapon/ENUM_WeaponState Enum" :default "NewEnumerator0"))
  (bind _skeletalmesh (`self.SkeletalMesh`))
  (bind _skeletalmesh_2 (`self.SkeletalMesh`))
  (bind _output_get (set `self.Weapon State` `New WeaponState`))
  (switch `/Game/Blueprints/Gameplay/Player/Equipment/Weapon/ENUM_WeaponState` _output_get
    (:`NewEnumerator0`
      (`PrimitiveComponent.SetCollisionProfileName` (`self.Sphere`) "OverlapAllDynamic" true)
      (`PrimitiveComponent.SetSimulatePhysics` _skeletalmesh true)
      (`PrimitiveComponent.SetCollisionProfileName` _skeletalmesh "DroppedWeapon" true)
      (`PrimitiveComponent.SetCastShadow` (`self.SkeletalMesh`) true))
    (:`NewEnumerator1`
      (`PrimitiveComponent.SetCollisionEnabled` (`self.Sphere`) "NoCollision")
      (`PrimitiveComponent.SetSimulatePhysics` _skeletalmesh_2 false)
      (`PrimitiveComponent.SetCollisionEnabled` _skeletalmesh_2 "NoCollision")
      (`SceneComponent.ResetRelativeTransform` _skeletalmesh_2)
      (`PrimitiveComponent.SetCastShadow` (`self.SkeletalMesh`) false))))

(fn `Show Mesh`
  (`SceneComponent.SetVisibility` (`self.SkeletalMesh`) true true))

(fn `Spread Trace`
  (params (InputTrace :type "Vector Structure"))
  (returns (SpreadTrace :type "Vector Structure"))
  (bind _returnvalue (* (`self.Spread`) 0.1))
  (bind _returnvalue_2 (* (`self.MinSpread`) _returnvalue))
  (bind _returnvalue_3 (* (`self.MaxSpread`) _returnvalue))
  (return (`KismetMathLibrary.MakeVector` (+ (.x InputTrace) (`KismetMathLibrary.RandomFloatInRange` _returnvalue_2 _returnvalue_3)) (+ (.y InputTrace) (`KismetMathLibrary.RandomFloatInRange` _returnvalue_2 _returnvalue_3)) (+ (.z InputTrace) (`KismetMathLibrary.RandomFloatInRange` _returnvalue_2 _returnvalue_3)))))

(fn `Update Recoil Pos`
  (params (Pitch :type "Float (double-precision)") (Yaw :type "Float (double-precision)"))
  (bind _returnvalue (`GameplayStatics.GetPlayerController` 0))
  (`PlayerController.AddPitchInput` _returnvalue Pitch)
  (`PlayerController.AddYawInput` _returnvalue Yaw))

(fn `UserConstructionScript`
  (bind _skeletalmesh (`self.SkeletalMesh`))
  (bind _weapon_mesh (`self.Weapon Mesh`))
  (`parent.UserConstructionScript`)
  (`/Engine/EditorBlueprintResources/StandardMacros.IsValid` _weapon_mesh
    (:`Is Valid`
      (`SkinnedMeshComponent.SetSkinnedAssetAndUpdate` _skeletalmesh _weapon_mesh true))
    (:`Is Not Valid`
      (`SkinnedMeshComponent.SetSkinnedAssetAndUpdate` _skeletalmesh "/Engine/EngineMeshes/SkeletalCube.SkeletalCube" true))))