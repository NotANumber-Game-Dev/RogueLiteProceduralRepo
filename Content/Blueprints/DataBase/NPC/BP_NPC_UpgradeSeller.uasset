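; NPC upgrade shop that offers randomized BP_PlayerModifier upgrades to the player.
; BeginPlay fills the UpgradeToSell array with randomized modifiers.
; ExecUIRelated creates WBP_NPC_Upgrades once, passes it the first offer and binds three buttons, then on every call shows it, pauses the game and switches to UI input.
; AddToPlayer gives the selected modifier to BP_Player, rerolls that slot and reapplies modifiers, with no price check.
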(event `self.ReceiveBeginPlay`
  (`parent.ReceiveBeginPlay`)
  (`self.generateShop`))

(fn `addToPlayer`
  (params (index :type Integer))
  (bind _asbp_player (cast `/Game/Blueprints/Gameplay/Player/BP_Player` (`GameplayStatics.GetPlayerPawn` 0)))
  (`KismetArrayLibrary.Array_Add` (`/Game/Blueprints/Gameplay/Player/BP_Player.Modifiers` _asbp_player) (`|GetArrayItem` (`self.UpgradeToSell`) index))
  (`self.updateShop` index)
  (`/Game/Blueprints/Gameplay/Player/BP_Player.applyModifiers` _asbp_player))

(fn `ExecUIRelated`
  (bind _returnvalue (`GameplayStatics.GetPlayerController` 0))
  (`parent.ExecUIRelated`)
  (`|ExecutionSequence`
    (:`then_0`
      (`/Engine/EditorBlueprintResources/StandardMacros.DoOnce` false
        (:`Completed`
          (bind _returnvalue_2 (`|CreateWidget` "/Game/UI/WBP_NPC_Upgrades.WBP_NPC_Upgrades_C" (`GameplayStatics.GetPlayerController` 0)))
          (bind _output_get (set `self.UIRelated` _returnvalue_2))
          (`/Game/UI/WBP_NPC_Upgrades.Add Element Upgrade` _output_get (`|GetArrayItem` (`self.UpgradeToSell`)) 0)
          (add `Button.OnClicked` (`/Game/UI/Components/Button/WBP_Button.ButtonElement` (`/Game/UI/WBP_NPC_Upgrades.UpgradeElement` _output_get)) (`|CreateDelegate` :!event `Modifier1`))
          (add `Button.OnClicked` (`/Game/UI/Components/Button/WBP_Button.ButtonElement` (`/Game/UI/WBP_NPC_Upgrades.UpgradeElement_1` _output_get)) (`|CreateDelegate` :!event `Modifier2`))
          (add `Button.OnClicked` (`/Game/UI/Components/Button/WBP_Button.ButtonElement` (`/Game/UI/WBP_NPC_Upgrades.UpgradeElement_2` _output_get)) (`|CreateDelegate` :!event `Modifier3`)))))
    (:`then_1`
      (`UserWidget.AddToViewport` _returnvalue_2 0)
      (`GameplayStatics.SetGamePaused` true)
      (`WidgetBlueprintLibrary.SetInputMode_UIOnlyEx` _returnvalue _returnvalue_2)
      (set `PlayerController.bShowMouseCursor` true _returnvalue))))

(fn `generateShop`
  (bind _upgradetosell (`self.UpgradeToSell`))
  (for (_ _array_index) _upgradetosell
    (bind _returnvalue (`|GenericCreateObject` "/Game/Blueprints/Gameplay/Player/Equipment/Upgrade/BP_PlayerModifier.BP_PlayerModifier_C" "BP_NPC_UpgradeSeller"))
    (`KismetArrayLibrary.Array_Set` _upgradetosell _array_index _returnvalue)
    (`/Game/Blueprints/Gameplay/Player/Equipment/Upgrade/BP_PlayerModifier.setRandomValues` _returnvalue)))

(fn `Modifier1`
  (`self.addToPlayer` 0))

(fn `Modifier2`
  (`self.addToPlayer` 1))

(fn `Modifier3`
  (`self.addToPlayer` 2))

(fn `updateShop`
  (params (idex :type Integer))
  (bind _returnvalue (`|GenericCreateObject` "/Game/Blueprints/Gameplay/Player/Equipment/Upgrade/BP_PlayerModifier.BP_PlayerModifier_C" "BP_NPC_UpgradeSeller"))
  (`KismetArrayLibrary.Array_Set` (`self.UpgradeToSell`) idex _returnvalue)
  (`/Game/Blueprints/Gameplay/Player/Equipment/Upgrade/BP_PlayerModifier.setRandomValues` _returnvalue))

(fn `UserConstructionScript`
  (`parent.UserConstructionScript`))