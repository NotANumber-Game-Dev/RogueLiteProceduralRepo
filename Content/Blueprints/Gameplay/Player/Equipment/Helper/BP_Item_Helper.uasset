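; BP_Item_Helper is a healing pickup that the player interacts with to collect, and its use adds HP up to the player's maximum.
; On BeginPlay it enters the Dropped state and creates an inventory widget showing its icon.
; OnInteracted passes it to the player's PickUpHelper.
; SetHelperState switches between a physics-simulated Dropped item and an Equipped one with collision, mesh and decal turned off.
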(event `self.ReceiveBeginPlay`
  (`self.setHelperState` "NewEnumerator0")
  (bind _returnvalue (`|CreateWidget` "/Game/UI/Components/Game/Inventory/WBP_Inventory_Item.WBP_Inventory_Item_C"))
  (bind _output_get (set `self.Inventory UI` _returnvalue))
  (`/Game/UI/Components/Game/Inventory/WBP_Inventory_Item.Set Image` _output_get (`self.UI_ShowTexture`)))

(event `/Game/Blueprints/Gameplay/Player/InteractionInterface/InteractionInterface.OnInteracted`
  (params (Player :type "/Game/Blueprints/Gameplay/Player/BP_Player Object Reference"))
  (`/Game/Blueprints/Gameplay/Player/BP_Player.PickUpHelper` Player self))

(fn `HideMesh`
  (`SceneComponent.SetVisibility` (`self.SkeletalMesh`) false true))

(fn `setHelperState`
  (params (NewState :type "/Game/Blueprints/Gameplay/Player/Equipment/Helper/ENUM_Item_Helper Enum" :default "NewEnumerator0"))
  (bind _sphere (`self.Sphere`))
  (bind _skeletalmesh (`self.SkeletalMesh`))
  (bind _output_get (set `self.HelperState` NewState))
  (switch `/Game/Blueprints/Gameplay/Player/Equipment/Helper/ENUM_Item_Helper` _output_get
    (:`NewEnumerator0`
      (`PrimitiveComponent.SetCollisionProfileName` _sphere "OverlapAllDynamic" true)
      (`PrimitiveComponent.SetSimulatePhysics` _skeletalmesh true)
      (`PrimitiveComponent.SetCollisionProfileName` _skeletalmesh "DroppedWeapon" true))
    (:`NewEnumerator1`
      (`PrimitiveComponent.SetCollisionEnabled` _sphere "NoCollision")
      (`PrimitiveComponent.SetSimulatePhysics` _skeletalmesh false)
      (`PrimitiveComponent.SetCollisionEnabled` _skeletalmesh "NoCollision")
      (`self.HideMesh`)
      (`SceneComponent.SetVisibility` (`self.Decal`) false false))))

(fn `UseHelper`
  (bind _asbp_player (cast `/Game/Blueprints/Gameplay/Player/BP_Player` (`GameplayStatics.GetPlayerCharacter` 0)))
  (bind _output_get (set `/Game/Blueprints/Gameplay/Player/BP_Player.HP` (+ (`/Game/Blueprints/Gameplay/Player/BP_Player.HP` _asbp_player) (`self.addHP`)) _asbp_player))
  (bind _maxhp (`/Game/Blueprints/Gameplay/Player/BP_Player.MaxHp` _asbp_player))
  (if (> _output_get _maxhp)
    (set `/Game/Blueprints/Gameplay/Player/BP_Player.HP` _maxhp _asbp_player)))

(fn `UserConstructionScript`
  (`parent.UserConstructionScript`))