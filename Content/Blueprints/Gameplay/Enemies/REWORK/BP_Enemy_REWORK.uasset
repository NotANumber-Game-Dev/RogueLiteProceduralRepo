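; Reworked enemy character that spawns and carries a weapon, takes damage from player and turret bullets, and may drop the weapon on death.
; Tick dispatches an enum state machine, with many states still empty stubs.
; Vision alert enables a looping delayed turn toward the player, while shooting is defined but never called here.
; Work in progress: Patrolling jumps straight to the timed zero-gravity state, leaving patrol movement and box-trace player detection disconnected.
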(event `self.ReceiveBeginPlay`
  (bind _returnvalue (`|SpawnActorFromClass` (`self.Desired Weapon`) (`KismetMathLibrary.MakeTransform` (0.0 0.0 0.0)) "Undefined" "OverrideRootScale" self null))
  (bind _output_get (set `self.Weapon` _returnvalue))
  (`self.K2_AttachToComponent` _output_get (`self.WeaponPosition`) "None" "SnapToTarget" "SnapToTarget" "SnapToTarget" true)
  (`/Game/Blueprints/Gameplay/Player/Equipment/Weapon/BP_Item_Weapon.Show Mesh` _output_get)
  (`/Game/Blueprints/Gameplay/Player/Equipment/Weapon/BP_Item_Weapon.setWeaponState` _output_get "NewEnumerator1")
  (`self.Should Rotate`)
  (`self.Find Random Patrol Point`))

(event `Should Rotate`
  (if (`self.CanRotate`)
    (set `self.Should Rotate to Player` true)
    (`self.Face Player`)
    (else
      (set `self.Should Rotate to Player` false)))
  (`KismetSystemLibrary.Delay` 0.001)
  (`self.Should Rotate`))

(event `self.ReceiveTick`
  (params (DeltaSeconds :type "Float (single-precision)"))
  (bind _output_get (set `self.Delta Seconds` DeltaSeconds))
  (set `self.Seconds Elapsed` (+ _output_get (`self.Seconds Elapsed`)))
  (`|ExecutionSequence`
    (:`then_0`
      (switch `/Game/Blueprints/Gameplay/Enemies/REWORK/ENUM_ENEMY_STATES` (`self.State`)
        (:`NewEnumerator0`
          (`self.StateIdle`))
        (:`NewEnumerator1`
          (`self.StateVisionAlert`))
        (:`NewEnumerator2`
          (`self.StateAttacking`))
        (:`NewEnumerator3`
          (`self.StateRunning`))
        (:`NewEnumerator4`
          (`self.StatePatroling`))
        (:`NewEnumerator5`
          (`self.StateRotating`))
        (:`NewEnumerator6`
          (`self.StateHealing`))
        (:`NewEnumerator7`
          (`self.StateHidding`))
        (:`NewEnumerator8`
          (`self.StateSoundAlert`))
        (:`NewEnumerator9`
          (`self.StateDead`))
        (:`NewEnumerator10`
          (`self.StateSearchPlayerArea`))
        (:`NewEnumerator11`
          (`self.StateThrowingGranade`))
        (:`NewEnumerator12`
          (`self.State Hited by Gravitatory Gadget`))))
    (:`then_1`
      (if (`self.Debug`)
        (`|ExecutionSequence`
          (:`then_0`
            (`KismetSystemLibrary.PrintString` (`KismetStringLibrary.Concat_StrStr` (`KismetStringLibrary.Concat_StrStr` (`KismetSystemLibrary.GetDisplayName` self) " /// ") (`|GetEnumeratorNameAsString` (`self.State`))) true false (struct :`G` 0.66 :`B` 1.0 :`A` 1.0) (`self.Delta Seconds`)))
          (:`then_1`
            (if (`self.ResetPatrolPosition`)
              (set `self.ResetPatrolPosition` false)
              (`self.Find Random Patrol Point`))))))))

(event `Delay`
  (params (Duration :type "Float (double-precision)"))
  (`KismetSystemLibrary.Delay` Duration))

(event `Find New Patrol With Delay`
  (params (Duration :type "Float (double-precision)"))
  (`KismetSystemLibrary.Delay` Duration)
  (`self.Find Random Patrol Point`))

(event `DelayInGravity`
  (params (Duration :type "Float (double-precision)"))
  (`KismetSystemLibrary.Delay` Duration)
  (set `CharacterMovementComponent.GravityScale` 1.0 (`self.CharacterMovement`))
  (set `self.State` "NewEnumerator1"))

(event `self.CapsuleComponent.OnComponentBeginOverlap`
  (params (OverlappedComponent :type "PrimitiveComponent Object Reference") (OtherActor :type "Actor Object Reference") (OtherComp :type "PrimitiveComponent Object Reference") (OtherBodyIndex :type Integer) (bFromSweep :type Boolean) (SweepResult :type "HitResult Structure (by ref)"))
  (bind _asbp_bullet (cast `/Game/Blueprints/Gameplay/Player/Equipment/Bullet/BP_Bullet` OtherActor))
  (if true
    (bind _whoshoted (`/Game/Blueprints/Gameplay/Player/Equipment/Bullet/BP_Bullet.WhoShoted` _asbp_bullet))
    (bind _asbp_player (cast `/Game/Blueprints/Gameplay/Player/BP_Player` _whoshoted)
      (:`then`
        (bind _output_get (set `self.HP` (- (`self.HP`) (`/Game/Blueprints/Gameplay/Player/Equipment/Weapon/BP_Item_Weapon.Damage Points` (`|GetArrayItem` (`/Game/Blueprints/Gameplay/Player/BP_Player.WeaponSlot` _asbp_player) (`/Game/Blueprints/Gameplay/Player/BP_Player.CurrentWeaponSlot` _asbp_player))))))
        (`KismetSystemLibrary.PrintString` (`KismetStringLibrary.Conv_IntToString` _output_get) false false))
      (:`CastFailed`
        (bind _asbp_pawn_turret (cast `/Game/Blueprints/Gameplay/Player/Equipment/Gadget/Turrent/BP_Pawn_Turret` _whoshoted))
        (bind _output_get_2 (set `self.HP` (- (`self.HP`) (`/Game/Blueprints/Gameplay/Player/Equipment/Weapon/BP_Item_Weapon.Damage Points` (`/Game/Blueprints/Gameplay/Player/Equipment/Gadget/Turrent/BP_Pawn_Turret.Weapon Asigned` _asbp_pawn_turret)))))
        (`KismetSystemLibrary.PrintString` (`KismetStringLibrary.Conv_IntToString` _output_get_2) true false)))
    (if (<= (`self.HP`) 0)
      (`self.K2_DestroyActor`)
      (if (> (`self.Drop Probability`) (`KismetMathLibrary.RandomFloatInRange` 0.0 100.0))
        (`/Game/Blueprints/Gameplay/Player/Equipment/Weapon/BP_Item_Weapon.setWeaponState` (`self.Weapon`) "NewEnumerator0")
        (else
          (`self.K2_DestroyActor` (`self.Weapon`))))
      (else
        (set `self.State` "NewEnumerator1")))
    (else
      (cast `/Game/Blueprints/Gameplay/Player/Equipment/Bullet/BP_GravityBullet` OtherActor)
      (if true
        (set `self.State` "NewEnumerator12")))))

(fn `Check if Seeing Player`
  (bind _shooting_camera (`self.Shooting Camera`))
  (bind _returnvalue (`SceneComponent.K2_GetComponentRotation` _shooting_camera))
  (bind _returnvalue_2 (`SceneComponent.K2_GetComponentLocation` _shooting_camera))
  (bind _outhits (`KismetSystemLibrary.BoxTraceMulti` :`Start` _returnvalue_2 :`End` (+ _returnvalue_2 (* (`KismetMathLibrary.GetForwardVector` _returnvalue) 500.0)) :`HalfSize` (100.0 100.0 100.0) :`Orientation` _returnvalue :`TraceChannel` "TraceTypeQuery2" :`DrawDebugType` "ForOneFrame"))
  (for _array_element _outhits
    (cast `/Game/Blueprints/Gameplay/Player/BP_Player` (`.HitActor` (`GameplayStatics.BreakHitResult` _array_element)))
    (set `self.State` "NewEnumerator1")))

(fn `Face Player`
  (if (`self.Should Rotate to Player`)
    (bind _asbp_controlled_main_game_instance (cast `/Game/Blueprints/GameModes/BP_ControlledMainGameInstance` (`GameplayStatics.GetGameInstance`)))
    (`/Game/Blueprints/GameModes/BP_ControlledMainGameInstance.LookAtPos` _asbp_controlled_main_game_instance self (`self.K2_GetActorLocation` (`GameplayStatics.GetPlayerPawn` 0)) 5.0)
    (else
      (`self.Should Rotate`))))

(fn `Find Random Patrol Point`
  (bind _patrol_radious (`self.Patrol Radious`))
  (bind _returnvalue (* (`KismetMathLibrary.GetPI`) 2.0 (`KismetMathLibrary.RandomFloat`)))
  (bind _output_get (set `self.PatrolPoint` (+ (`self.K2_GetActorLocation`) (`KismetMathLibrary.MakeVector` (* (`KismetMathLibrary.Sin` _returnvalue) _patrol_radious) (* _patrol_radious (`KismetMathLibrary.Cos` _returnvalue))))))
  (`KismetSystemLibrary.PrintString` (`KismetStringLibrary.Conv_VectorToString` _output_get)))

(fn `Go to Player`
  (`AIController.MoveToLocation` (`AIBlueprintHelperLibrary.GetAIController` self) (`self.K2_GetActorLocation` (`GameplayStatics.GetPlayerPawn` 0)) 60.0 true true false true null true))

(fn `Go To Random Patrol Point`
  (returns (Succes :type "EPathFollowingRequestResult Enum"))
  (bind _returnvalue (`AIBlueprintHelperLibrary.GetAIController` self))
  (bind _returnvalue_2 (`AIController.MoveToLocation` _returnvalue (`self.PatrolPoint`) 60.0 true true false (`AIController.bAllowStrafe` _returnvalue) null true))
  (`KismetSystemLibrary.PrintString` (`|GetEnumeratorNameAsString` _returnvalue_2) true true (struct :`G` 0.66 :`B` 1.0 :`A` 1.0) (`self.Delta Seconds`))
  (return _returnvalue_2))

(fn `HealUp`
  (set `self.HP` (+ (`self.HP`) (/ (`self.Max_HP`) 3))))

(fn `RotateToPlayer`
  (params (`Can it` :type Boolean))
  (set `self.CanRotate` `Can it`))

(fn `ShootPlayer`
  (if (>= (`self.Seconds Elapsed`) (`/Game/Blueprints/Gameplay/Player/Equipment/Weapon/BP_Item_Weapon.Fire Rate` (`self.Weapon`)))
    (set `self.Seconds Elapsed` 0.0)
    (bind _return (`/Game/Blueprints/Gameplay/Player/Equipment/Weapon/BP_Item_Weapon.Get Current Clip Ammo` (`self.Weapon`)))
    (if (<= _return 0)
      (`/Game/Blueprints/Gameplay/Player/Equipment/Weapon/BP_Item_Weapon.Reload` (`self.Weapon`) false))
    (`/Game/Blueprints/Gameplay/Player/Equipment/Weapon/BP_Item_Weapon.Fire` (`self.Weapon`) (`self.Shooting Camera`) false self)
    (`GameplayStatics.PlaySoundAtLocation` null (`self.K2_GetActorLocation`) (struct) 1.0 1.0 0.0 null null null)))

(fn `State Hited by Gravitatory Gadget`
  (set `CharacterMovementComponent.GravityScale` 0.0 (`self.CharacterMovement`))
  (`self.DelayInGravity` 4.0))

(fn `StateAttacking`)

(fn `StateDead`)

(fn `StateHealing`
  (`self.HealUp`))

(fn `StateHidding`)

(fn `StateIdle`
  (set `self.State` "NewEnumerator4"))

(fn `StatePatroling`
  (set `self.State` "NewEnumerator12"))

(fn `StateRotating`)

(fn `StateRunning`)

(fn `StateSearchPlayerArea`)

(fn `StateSoundAlert`)

(fn `StateThrowingGranade`)

(fn `StateVisionAlert`
  (`self.RotateToPlayer` true)
  (`self.StateAttacking`))

(fn `UpdateWalkSpeed`
  (params (`Max Walk Speed` :type "Float (double-precision)"))
  (set `CharacterMovementComponent.MaxWalkSpeed` `Max Walk Speed` (`self.CharacterMovement`)))

(fn `UserConstructionScript`
  (`SkinnedMeshComponent.SetSkinnedAssetAndUpdate` (`self.Mesh`) (`self.Enemy Mesh`) true)
  (set `AIController.bAllowStrafe` true (`AIBlueprintHelperLibrary.GetAIController` self))
  (set `self.Max_HP` (`self.HP`)))