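; BP_Button is a one-shot interactable button prop.
; Its OnInteracted event marks it as activated, sets ShowTooltip to true and disables collision on its Sphere component.
; The event graph holds no other active logic, and the construction script only calls its parent.
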(event `/Game/Blueprints/Gameplay/Player/InteractionInterface/InteractionInterface.OnInteracted`
  (params (Player :type "/Game/Blueprints/Gameplay/Player/BP_Player Object Reference"))
  (set `self.Has Been Activated` true)
  (set `self.Show Tooltip` true)
  (`PrimitiveComponent.SetCollisionEnabled` (`self.Sphere`) "NoCollision"))

(fn `UserConstructionScript`
  (`parent.UserConstructionScript`))