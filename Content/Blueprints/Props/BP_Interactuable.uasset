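; BP_Interactuable is an interactable prop that drives the player's HUD tooltip for interaction prompts.
; On entering interaction range, it stores the player and, if ShowTooltip is set, shows InteractionTooltip joined with Name plus an interact button.
; On exiting range, it hides that tooltip through the stored player's HUDWidget, under the same flag.
; It contains no range detection or interaction logic in these graphs.
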(event `/Game/Blueprints/Gameplay/Player/InteractionInterface/InteractionInterface.OnIteractionRangeEntered`
  (params (Player :type "/Game/Blueprints/Gameplay/Player/BP_Player Object Reference"))
  (if (`self.Show Tooltip`)
    (bind _output_get (set `self.Player` Player))
    (bind _hud_widget (`/Game/Blueprints/Gameplay/Player/BP_Player.HUD_Widget` _output_get))
    (`/Game/UI/WBP_HUD.Set Tooltip` _hud_widget (`KismetTextLibrary.Conv_StringToText` (`KismetStringLibrary.Concat_StrStr` (`KismetStringLibrary.Concat_StrStr` (`KismetTextLibrary.Conv_TextToString` (`self.Interaction Tooltip`)) " ") (`KismetTextLibrary.Conv_TextToString` (`self.Name`)))) true)
    (`/Game/UI/WBP_HUD.Show Tooltip` _hud_widget)))

(event `/Game/Blueprints/Gameplay/Player/InteractionInterface/InteractionInterface.OnInteractionRangeExited`
  (if (`self.Show Tooltip`)
    (`/Game/UI/WBP_HUD.Hide Tooltip` (`/Game/Blueprints/Gameplay/Player/BP_Player.HUD_Widget` (stale `/Game/Blueprints/Gameplay/Player/InteractionInterface/InteractionInterface.OnIteractionRangeEntered` _output_get)))
    (`/Game/UI/WBP_HUD.Hide Tooltip` (`/Game/Blueprints/Gameplay/Player/BP_Player.HUD_Widget` (`self.Player`)))))

(fn `UserConstructionScript`)