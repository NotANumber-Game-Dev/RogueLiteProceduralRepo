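; Blinking LED light prop for the maze that toggles its point light on and off.
; The construction script caches the light's authored intensity as the on value.
; Tick drives a short fixed Delay into a FlipFlop that alternates between that intensity and zero.
; A random-range node is left unconnected, so the blink rate does not vary.
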(event `self.ReceiveTick`
  (params (DeltaSeconds :type "Float (single-precision)"))
  (`KismetSystemLibrary.Delay` 0.2)
  (`/Engine/EditorBlueprintResources/StandardMacros.FlipFlop`
    (:`A`
      (`LightComponent.SetIntensity` (`self.PointLighta`) (`self.Intensity`)))
    (:`B`
      (`LightComponent.SetIntensity` (`self.PointLighta`) 0.0))))

(fn `UserConstructionScript`
  (set `self.Intensity` (`LightComponentBase.Intensity` (`self.PointLighta`))))