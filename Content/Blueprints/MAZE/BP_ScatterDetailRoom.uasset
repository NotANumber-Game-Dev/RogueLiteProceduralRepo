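; Maze room detail scatterer that fills a box area with randomly placed, yaw-rotated instanced static meshes.
; On construction and BeginPlay it reads radius, count and trace range from XML, then picks seeded points, optionally clustered toward the center.
; Sphere traces reject occupied points, with DoN-limited retries.
; Tick hides the Billboard and its children when the player is over two BP_MazeGenerator squares away.
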(event `self.ReceiveBeginPlay`
  (bind _outactors (`GameplayStatics.GetAllActorsOfClass` "/Game/Blueprints/MAZE/BP_MazeGenerator.BP_MazeGenerator_C"))
  (set `self.MazeInfo` (`|GetArrayItem` _outactors))
  (`self.InstanceObjects`))

(event `self.ReceiveTick`
  (params (DeltaSeconds :type "Float (single-precision)"))
  (bind _returnvalue (`GameplayStatics.GetPlayerPawn` 0))
  (bind _billboard (`self.Billboard`))
  (`/Engine/EditorBlueprintResources/StandardMacros.IsValid` _returnvalue
    (:`Is Valid`
      (if (> (`KismetMathLibrary.VSize` (- (`self.K2_GetActorLocation`) (`self.K2_GetActorLocation` _returnvalue))) (* (`MazeGenerator.getSizeSquare` (`self.MazeInfo`)) 2.0))
        (`SceneComponent.SetVisibility` _billboard false true)
        (else
          (`SceneComponent.SetVisibility` _billboard true true))))))

(fn `InstanceObjects`
  (bind _instanced_meshes (`self.Instanced Meshes`))
  (bind _meshes_to_spawn (`self.Meshes to spawn`))
  (bind _radius (`self.Radius`))
  (bind _random_seed (`self.Random Seed`))
  (bind _collision_trace_range (`self.Collision Trace Range`))
  (bind _returnvalue (/ _collision_trace_range 5.0))
  (bind _returnvalue_2 (* _radius -1.0))
  (bind _returnvalue_3 (+ (`self.K2_GetActorLocation`) (`self.Spawn Point`)))
  (bind _returnvalue_4 (`KismetMathLibrary.RandomFloatInRangeFromStream` 1.0 (`KismetMathLibrary.SelectFloat` 1.8 1.0 (`self.Cluster Around Center`)) _random_seed))
  (bind _output (`|GetArrayItem` _instanced_meshes (`KismetMathLibrary.RandomIntegerInRangeFromStream` 0 (`KismetArrayLibrary.Array_Length` _instanced_meshes) (`self.Random Seed`))))
  (`ReadXMLLevelDetail.ReadXmlFile` (`KismetStringLibrary.Concat_StrStr` (`KismetSystemLibrary.GetProjectContentDirectory`) (`self.Xml Path`)))
  (bind _var (`ReadXMLLevelDetail.getRootAttributes`))
  (set `self.RootAttributes` _var)
  (bind _var_2 (`ReadXMLLevelDetail.getTag`))
  (set `self.XMLTags` _var_2)
  (bind _var_3 (`ReadXMLLevelDetail.getChildTag`))
  (set `self.XMLChildren Tags` _var_3)
  (bind _var_4 (`ReadXMLLevelDetail.getContent`))
  (set `self.XMLContent` _var_4)
  (bind _var_5 (`ReadXMLLevelDetail.getChildContent`))
  (set `self.XMLChild Content` _var_5)
  (set `self.Cluster Around Center` (== (`|GetArrayItem` (`self.RootAttributes`) 1) "true"))
  (bind _output_get (set `self.Radius` (`KismetStringLibrary.Conv_StringToDouble` (`|GetArrayItem` (`self.XMLContent`) 1))))
  (bind _output_get_2 (set `self.Collision Trace Range` (`KismetStringLibrary.Conv_StringToDouble` (`|GetArrayItem` (`self.XMLContent`) 2))))
  ;[1 1 1] Spawn Area Size Control
  (`BoxComponent.SetBoxExtent` (`self.Radius_Vis`) (`KismetMathLibrary.MakeVector` _output_get _output_get _output_get_2) true)
  ;[1 1 1] Create instanced static mesh components to use as templates, once for each mesh type
  (set `self.Number of meshes` (`KismetStringLibrary.Conv_StringToInt` (`|GetArrayItem` (`self.XMLContent`) 4)))
  (for _index (range (+ (`KismetArrayLibrary.Array_Length` _meshes_to_spawn) 1))
    (bind _returnvalue_5 (`AddComponent|NODE_AddInstancedStaticMeshComponent-0`))
    (`StaticMeshComponent.SetStaticMesh` _returnvalue_5 (`|GetArrayItem` _meshes_to_spawn _index))
    (`KismetArrayLibrary.Array_Add` (`self.Instanced Meshes`) _returnvalue_5))
  (for _ (range 1 (+ (`KismetMathLibrary.Clamp` (`self.Number of meshes`) 1 50) 1))
    ;[1 1 1] Checking collision between the object to spawn and anything around
    (set `self.Spawn Point` (`KismetMathLibrary.MakeVector` (/ (`KismetMathLibrary.RandomFloatInRangeFromStream` _returnvalue_2 _radius _random_seed) _returnvalue_4) (/ (`KismetMathLibrary.RandomFloatInRangeFromStream` _returnvalue_2 _radius _random_seed) _returnvalue_4) (`KismetMathLibrary.RandomFloatInRangeFromStream` -15.0 -4.0 _random_seed)) :!label _label)
    (bind (_outhit _returnvalue_6) (`KismetSystemLibrary.SphereTraceSingle` :`Start` (+ (`KismetMathLibrary.MakeVector` 0.0 0.0 _collision_trace_range) _returnvalue_3) :`End` (+ (`KismetMathLibrary.MakeVector` 0.0 0.0 (/ _returnvalue 1.0)) _returnvalue_3) :`Radius` _returnvalue :`TraceChannel` "TraceTypeQuery1" :`bTraceComplex` true :`TraceColor` (struct :`R` 1.0) :`TraceHitColor` (struct :`G` 1.0) :`DrawTime` 0.1))
    (if _returnvalue_6
      (`/Engine/EditorBlueprintResources/StandardMacros.Do N` 0 :!label _label_2
        (:`Exit`
          (goto _label)))
      (else
        (`|ExecutionSequence`
          (:`then_0`
            (goto _label_2 :!via `Reset`))
          (:`then_1`
            (`/Engine/EditorBlueprintResources/StandardMacros.IsValid` _output
              (:`Is Valid`
                (`InstancedStaticMeshComponent.AddInstance` _output (`KismetMathLibrary.MakeTransform` (- (`self.Spawn Point`) (0.0 0.0 -10.0)) (`KismetMathLibrary.MakeRotator` 0.0 0.0 (`KismetMathLibrary.RandomFloatInRangeFromStream` 0.0 360.0 (`self.Random Seed`)))))))))))))

(fn `UserConstructionScript`
  (`self.InstanceObjects`))