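; Interactable scrapper machine that presents its scrapper UI on an in-world widget component.
; BeginPlay caches the 3D-space scrapper widget; when a player enters interaction range, their equipment is added to inventory and that widget is shown.
; An older screen-space version remains: its widget is still created, but the viewport, pause and UI-only input logic is disconnected.
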(event `self.ReceiveBeginPlay`
  (bind _aswbp_scrapper_3dspace (cast `/Game/UI/Components/Scrapper_Oriol/WBP_Scrapper_3DSpace` (`WidgetComponent.GetWidget` (`self.Widget`))))
  (set `self. Scrapper 3DSpace` _aswbp_scrapper_3dspace)
  ;[1 1 1] Old
  (bind _returnvalue (`|CreateWidget` "/Game/UI/Components/Scrapper_Oriol/WBP_Scrapper.WBP_Scrapper_C"))
  (set `self.Scraper_Widget` _returnvalue))

(event `self.ReceiveActorBeginOverlap`
  (params (OtherActor :type "Actor Object Reference")))

(event `/Game/Blueprints/Gameplay/Player/InteractionInterface/InteractionInterface.OnInteracted`
  (params (Player :type "/Game/Blueprints/Gameplay/Player/BP_Player Object Reference"))
  ;[1 1 1] Old
)

(event `/Game/Blueprints/Gameplay/Player/InteractionInterface/InteractionInterface.OnIteractionRangeEntered`
  (params (Player :type "/Game/Blueprints/Gameplay/Player/BP_Player Object Reference"))
  (`/Game/Blueprints/Gameplay/Player/BP_Player.AddEquippementToInventory` Player)
  (`/Game/UI/Components/Scrapper_Oriol/WBP_Scrapper_3DSpace.Show` (`self. Scrapper 3DSpace`)))

(fn `UserConstructionScript`)