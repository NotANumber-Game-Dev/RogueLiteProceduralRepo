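; Melee weapon item whose Fire function detects enemies inside a hit box, with no damage applied yet.
; The box has collision off from BeginPlay and switches to overlap only for the duration of Fire.
; Fire filters overlapping components to BP_Enemy_REWORK capsules and records hits in EnemyHit, with a duplicate check and a debug print on the first.
; The list is cleared once the box is disabled again.
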(event `self.ReceiveBeginPlay`
  (`parent.ReceiveBeginPlay`)
  (`PrimitiveComponent.SetCollisionEnabled` (`self.Box`) "NoCollision"))

(fn `Fire`
  (params (`Player Camera` :type "CameraComponent Object Reference") (isPlayer :type Boolean) (WhoShoted :type "Pawn Object Reference"))
  (locals (Enemy_hit :type "Array of /Game/Blueprints/Gameplay/Enemies/REWORK/BP_Enemy_REWORK Object Reference"))
  (bind _box (`self.Box`))
  (bind _enemy_hit (`local.Enemy_hit`))
  (`PrimitiveComponent.SetCollisionProfileName` _box "OverlapAllDynamic" true)
  (for _array_element (`PrimitiveComponent.GetOverlappingComponents` _box)
    (bind _ascapsule_collision (cast `CapsuleComponent` _array_element))
    (bind _asbp_enemy_rework (cast `/Game/Blueprints/Gameplay/Enemies/REWORK/BP_Enemy_REWORK` (`ActorComponent.GetOwner` _ascapsule_collision)))
    (if (== (`KismetArrayLibrary.Array_Length` _enemy_hit) 0)
      (`KismetArrayLibrary.Array_Add` _enemy_hit)
      (`KismetSystemLibrary.PrintString` "cac")
      (else
        (for _array_element_2 _enemy_hit
          (if (== _array_element_2 _asbp_enemy_rework)
            (break)))
        (`KismetArrayLibrary.Array_Add` _enemy_hit))))
  (`PrimitiveComponent.SetCollisionProfileName` _box "NoCollision" false)
  (`KismetArrayLibrary.Array_Clear` _enemy_hit))

(fn `UserConstructionScript`
  (`parent.UserConstructionScript`))