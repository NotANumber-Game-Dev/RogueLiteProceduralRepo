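; Maze generator actor that, in this graph, handles player spawn placement and stores an XML file path, with no maze-building logic.
; On BeginPlay it gathers all BP_SpawnPlayer and BP_Player actors, then teleports the first player to each spawn point within RadiusToSpawn.
; The loop has no break and measures from the player's current position, so successive moves can chain.
; SetXmlFile only sets XmlPath.
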(event `self.ReceiveBeginPlay`
  (bind _outactors (`GameplayStatics.GetAllActorsOfClass` "/Game/Blueprints/MAZE/BP_SpawnPlayer.BP_SpawnPlayer_C"))
  (bind _output_get (set `self.Possible Spawn Point` _outactors))
  (bind _outactors_2 (`GameplayStatics.GetAllActorsOfClass` "/Game/Blueprints/Gameplay/Player/BP_Player.BP_Player_C"))
  (bind _output_get_2 (set `self.Player` _outactors_2))
  (for _array_element _output_get
    (bind _output (`|GetArrayItem` _output_get_2))
    (if (<= (`self.GetDistanceTo` _array_element _output) (`self.Radius to Spawn`))
      (`self.K2_SetActorLocation` _output (`self.K2_GetActorLocation` _array_element) false true))))

(event `self.ReceiveTick`
  (params (DeltaSeconds :type "Float (single-precision)")))

(fn `setXmlFile`
  (params (Path :type String))
  (set `self.Xml Path` Path))

(fn `UserConstructionScript`)