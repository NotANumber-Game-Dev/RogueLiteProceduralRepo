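; Item spawner that, on BeginPlay, may spawn one random weapon item at its own transform.
; A random roll must meet or exceed ProbSpawn, so higher values make a spawn less likely.
; The class is picked at random from the SpawnItemWeapon array and spawns with collision adjustment, always spawning.
; The spawned actor then receives a random rotation on all three axes.
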(event `self.ReceiveBeginPlay`
  (bind _spawnitemweapon (`self.SpawnItemWeapon`))
  (if (>= (`KismetMathLibrary.RandomIntegerInRange` 0 100) (`self.Prob Spawn`))
    (bind _returnvalue (`|SpawnActorFromClass` (`|GetArrayItem` _spawnitemweapon (`KismetMathLibrary.RandomIntegerInRange` 0 (- (`KismetArrayLibrary.Array_Length` _spawnitemweapon) 1))) (`self.GetTransform`) "AdjustIfPossibleButAlwaysSpawn" "OverrideRootScale" null null))
    (`self.K2_SetActorRotation` _returnvalue (`KismetMathLibrary.MakeRotator` (`KismetMathLibrary.RandomFloatInRange` 45.0 360.0) (`KismetMathLibrary.RandomFloatInRange` 45.0 360.0) (`KismetMathLibrary.RandomFloatInRange` 45.0 360.0)) false)))

(fn `UserConstructionScript`)