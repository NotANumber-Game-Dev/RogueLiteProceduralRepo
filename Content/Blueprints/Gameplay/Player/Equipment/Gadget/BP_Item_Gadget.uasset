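; Base pickup item for player gadgets, with empty Fire, Start and UpdateHUD functions.
; It starts Dropped as a physics object with an inventory widget; interaction hands it to the player and adds it to the mission.
; SetGadgetState switches collision, physics and visibility, ticking on cooldown but not when equipped or stored.
; Equipped, stored and cooldown states hide and attach it to the viewmodel socket, except turrets, which use Instanciable and enable surveillance-radius overlaps.
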(event `self.ReceiveBeginPlay`
  (`self.setGadgetState` "NewEnumerator0")
  (bind _returnvalue (`|CreateWidget` "/Game/UI/Components/Game/Inventory/WBP_Inventory_Item.WBP_Inventory_Item_C"))
  (bind _output_get (set `self.Inventory UI` _returnvalue))
  (`/Game/UI/Components/Game/Inventory/WBP_Inventory_Item.Set Image` _output_get (`self.UI_ShowTexture`)))

(event `/Game/Blueprints/Gameplay/Player/InteractionInterface/InteractionInterface.OnInteracted`
  (params (Player :type "/Game/Blueprints/Gameplay/Player/BP_Player Object Reference"))
  (`/Game/Blueprints/Gameplay/Player/BP_Player.PickUpGadget` Player self)
  ;[1 1 1] Afegir a missio
  (`self.AddItemToMission`))

(fn `Fire`)

(fn `hideMesh`
  (`SceneComponent.SetVisibility` (`self.SkeletalMesh`) false true))

(fn `setGadgetState`
  (params (NewGadgetState :type "/Game/Blueprints/Gameplay/Player/Equipment/Gadget/ENUM_GadgetStates Enum" :default "NewEnumerator0"))
  (bind _skeletalmesh (`self.SkeletalMesh`))
  (bind _skeletalmesh_2 (`self.SkeletalMesh`))
  (bind _skeletalmesh_3 (`self.SkeletalMesh`))
  (bind _output_get (set `self.GadgetState` NewGadgetState))
  (switch `/Game/Blueprints/Gameplay/Player/Equipment/Gadget/ENUM_GadgetStates` _output_get
    (:`NewEnumerator0`
      (`PrimitiveComponent.SetCollisionProfileName` (`self.Sphere`) "OverlapAllDynamic" true)
      (`PrimitiveComponent.SetSimulatePhysics` _skeletalmesh true)
      (`PrimitiveComponent.SetCollisionProfileName` _skeletalmesh "DroppedWeapon" true))
    (:`NewEnumerator1`
      (`self.SetActorTickEnabled` false :!label _label)
      (`PrimitiveComponent.SetCollisionEnabled` (`self.Sphere`) "NoCollision" :!label _label_2)
      (`PrimitiveComponent.SetSimulatePhysics` _skeletalmesh_3 false)
      (`PrimitiveComponent.SetCollisionEnabled` _skeletalmesh_3 "NoCollision")
      (`SceneComponent.ResetRelativeTransform` _skeletalmesh_3)
      (`self.hideMesh`)
      (bind _asbp_player (cast `/Game/Blueprints/Gameplay/Player/BP_Player` (`GameplayStatics.GetPlayerPawn` 0)))
      (bind _asbp_item_gadget_torret (cast `/Game/Blueprints/DataBase/Gadgets/BP_Item_Gadget_Torret` self)
        (:`then`
          (`self.K2_AttachToComponent` (`/Game/Blueprints/Gameplay/Player/BP_Player.Instanciable` _asbp_player) "None" "SnapToTarget" "SnapToTarget" "SnapToTarget")
          (set `PrimitiveComponent.bGenerateOverlapEvents` true (`/Game/Blueprints/DataBase/Gadgets/BP_Item_Gadget_Torret.RadiDeVigilancia` _asbp_item_gadget_torret)))
        (:`CastFailed`
          (`self.K2_AttachToComponent` (`/Game/Blueprints/Gameplay/Player/BP_Player.Viewmodel` _asbp_player) "weaponSocket" "SnapToTarget" "SnapToTarget" "SnapToTarget"))))
    (:`NewEnumerator2`
      (`PrimitiveComponent.SetCollisionEnabled` (`self.Sphere`) "NoCollision")
      (`PrimitiveComponent.SetSimulatePhysics` _skeletalmesh_2 false)
      (`PrimitiveComponent.SetCollisionEnabled` _skeletalmesh_2 "NoCollision")
      (`SceneComponent.ResetRelativeTransform` _skeletalmesh_2)
      (`self.showMesh`))
    (:`NewEnumerator3`
      (goto _label))
    (:`NewEnumerator4`
      (`self.SetActorTickEnabled` true)
      (goto _label_2))))

(fn `showMesh`
  (`SceneComponent.SetVisibility` (`self.SkeletalMesh`) true true))

(fn `Start`)

(fn `UpdateHUD`
  (params (HUD :type "/Game/UI/WBP_HUD Object Reference") (Player :type "/Game/Blueprints/Gameplay/Player/BP_Player Object Reference")))

(fn `UserConstructionScript`
  (bind _skeletalmesh (`self.SkeletalMesh`))
  (bind _gadgetmesh (`self.GadgetMesh`))
  (`parent.UserConstructionScript`)
  (`/Engine/EditorBlueprintResources/StandardMacros.IsValid` _gadgetmesh
    (:`Is Valid`
      (`SkinnedMeshComponent.SetSkinnedAssetAndUpdate` _skeletalmesh _gadgetmesh true))
    (:`Is Not Valid`
      (`SkinnedMeshComponent.SetSkinnedAssetAndUpdate` _skeletalmesh "/Engine/EngineMeshes/SkeletalCube.SkeletalCube" true))))